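; Game mode for a turn-based, dice-driven tile tactics game between human and computer heroes.
; BeginPlay spawns both teams on random generator tiles and interleaves them into a round-robin list, outlining the active hero.
; Computer turns spend dice as movement tokens toward a human target, then as attack damage, chained through move and damage callbacks.
; Each turn change first checks both sides for survivors and opens the final screen when either is wiped out.
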(event `self.ReceiveBeginPlay`
  (bind _gamestateref (`self.GameStateRef`))
  ;[1 1 1] Spawn players and start turn
  (bind _asbp_top_down_controller (cast `/Game/Blueprints/Core/BP_TopDownController` (`GameplayStatics.GetPlayerController` 0)))
  (set `self.PlayerControlerRef` _asbp_top_down_controller)
  (bind _asgs_state (cast `/Game/GS_State` (`GameplayStatics.GetGameState`)))
  (set `self.GameStateRef` _asgs_state)
  (bind _returnvalue (`GameplayStatics.GetActorOfClass` "/Game/Blueprints/Grid/BP_Generator.BP_Generator_C"))
  (set `self.TileGeneratorRef` _returnvalue)
  (bind _randomint (`self.GetRandomTiles` (`/Game/GS_State.MaxPlayers` _gamestateref)))
  (bind _output_get (set `self.PlayerRandomTilesIndex` _randomint))
  (bind _randomint_2 (`self.GetRandomTiles` (`/Game/GS_State.MaxOpponents` _gamestateref)))
  (bind _output_get_2 (set `self.OpponentRandomTilesIndex` _randomint_2))
  (`self.SpawnActors` _output_get_2 (5.0 4.0) (`self.Opponents`) (0.0 90.0 0.0) (`BlueprintGameplayTagLibrary.GetTagName` (`BlueprintGameplayTagLibrary.MakeLiteralGameplayTag` (struct :`TagName` "Game.PlayerTag.Computer"))))
  (`self.SpawnActors` _output_get (18.0 4.0) (`self.Players`) (0.0 -90.0 0.0) (`BlueprintGameplayTagLibrary.GetTagName` (`BlueprintGameplayTagLibrary.MakeLiteralGameplayTag` (struct :`TagName` "Game.PlayerTag.Human"))))
  (`self.Init Players`)
  (`/Game/Blueprints/Player/BP_DefaultHero.StartTurn` (`self.CurrentPlayer`)))

(event `Init Players`
  (bind _players (`self.Players`))
  (bind _opponents (`self.Opponents`))
  ;[1 1 1] Suffle Players
  (if (> (`KismetArrayLibrary.Array_Length` _players) 0) :!label _label
    (`KismetArrayLibrary.Array_Add` (`self.RoundRobinPlayers`) (`|GetArrayItem` _players))
    (`KismetArrayLibrary.Array_Remove` (`self.Players`))
    (if (> (`KismetArrayLibrary.Array_Length` _opponents) 0)
      (`KismetArrayLibrary.Array_Add` (`self.RoundRobinPlayers`) (`|GetArrayItem` _opponents))
      (`KismetArrayLibrary.Array_Remove` (`self.Opponents`))
      (goto _label))
    (else
      (`self.SelectPlayer`))))

(event `SelectPlayer`
  (bind _output (`|GetArrayItem` (`self.RoundRobinPlayers`) (`self.CurrentPlayerIndex`)))
  ;[1 1 1] Select player
  (bind _output_get (set `self.CurrentPlayer` _output))
  (set `/Game/GS_State.CurrentPlayer` _output_get (`self.GameStateRef`))
  (`MeshComponent.SetOverlayMaterial` (`Character.Mesh` _output) "/Game/Materials/M_Outline.M_Outline"))

(event `NextTurn`
  ;[1 1 1] Turn change
  (`self.EvaluateFinish`)
  (if (`self.AnyOponentAlive`)
    (if (`self.AnyHeroAlive`)
      (`MeshComponent.SetOverlayMaterial` (`Character.Mesh` (`self.CurrentPlayer`)) null)
      (bind _result (`/Engine/EditorBlueprintResources/StandardMacros.IncrementInt` (`self.CurrentPlayerIndex`))
        (:`  `
          (if (>= _result (`KismetArrayLibrary.Array_Length` (`self.RoundRobinPlayers`)))
            (set `self.CurrentPlayerIndex` 0)
            (else
              (set `self.CurrentPlayerIndex` _result)))
          (`self.SelectPlayer`)
          (`self.TurnSelector`))))))

(event `TurnSelector`
  ;[1 1 1] Turn switcher
  (if (`KismetArrayLibrary.Array_Contains` (`Actor.Tags` (`self.CurrentPlayer`)) (`BlueprintGameplayTagLibrary.GetTagName` (`BlueprintGameplayTagLibrary.MakeLiteralGameplayTag` (struct :`TagName` "Game.PlayerTag.Computer"))))
    (`self.ComputerTurn`)
    (else
      (`self.HumanTurn`)
      (`/Game/Blueprints/Player/BP_DefaultHero.StartTurn` (`self.CurrentPlayer`)))))

(event `HumanTurn`)

(event `ComputerTurn`
  (bind _currentplayer (`self.CurrentPlayer`))
  ;[1 1 1] Computer turn
  (`/Game/Blueprints/Core/BP_TopDownController.AITurn` (`self.PlayerControlerRef`))
  (`/Game/Blueprints/Player/BP_DefaultHero.AddRandomForm` _currentplayer)
  (set `self.Tokens` 0)
  (`KismetArrayLibrary.Array_Clear` (`self.Dices`))
  (for _array_element (`/Game/Blueprints/Player/BP_DefaultHero.Character dice` _currentplayer)
    (if (> _array_element 0)
      (`KismetArrayLibrary.Array_Add` (`self.Dices`) _array_element)))
  (`self.DoAIAction`))

(event `EvaluateFinish`
  ;[1 1 1] Evaluate if the game is finished and eventually who won
  (set `self.AnyOponentAlive` false)
  (set `self.AnyHeroAlive` false)
  (bind _outactors (`GameplayStatics.GetAllActorsOfClassWithTag` "/Game/Blueprints/Player/BP_DefaultHero.BP_DefaultHero_C" (`BlueprintGameplayTagLibrary.GetTagName` (`BlueprintGameplayTagLibrary.MakeLiteralGameplayTag` (struct :`TagName` "Game.PlayerTag.Computer")))))
  (for _array_element _outactors
    (if (`/Game/Blueprints/Components/Health_System.IsAlive` (`/Game/Blueprints/Player/BP_DefaultHero.Health_System` _array_element))
      (set `self.AnyOponentAlive` true)
      (break)))
  (if (`self.AnyOponentAlive`)
    (bind _outactors_2 (`GameplayStatics.GetAllActorsOfClassWithTag` "/Game/Blueprints/Player/BP_DefaultHero.BP_DefaultHero_C" (`BlueprintGameplayTagLibrary.GetTagName` (`BlueprintGameplayTagLibrary.MakeLiteralGameplayTag` (struct :`TagName` "Game.PlayerTag.Human")))))
    (for _array_element_2 _outactors_2
      (if (`/Game/Blueprints/Components/Health_System.IsAlive` (`/Game/Blueprints/Player/BP_DefaultHero.Health_System` _array_element_2))
        (set `self.AnyHeroAlive` true)
        (break)))
    (if (`self.AnyHeroAlive`)
      (if (not (`self.AnyOponentAlive`))
        (`self.ShowFinalScreen` true))
      (else
        (`self.ShowFinalScreen` false)))
    (else
      (`self.ShowFinalScreen` false))))

(event `ComputerMove`
  (bind _currentplayer (`self.CurrentPlayer`))
  ;[1 1 1] Computer move
  (`/Game/Blueprints/Grid/BP_Generator.ComputerPathWay` (`self.TileGeneratorRef`) (`self.Tokens`))
  (add `/Game/Blueprints/Player/BP_DefaultHero.OnFollowPathEnded` _currentplayer (delegate `OnFollowPathEnded`))
  (`/Game/Blueprints/Player/BP_DefaultHero.FollowPath` _currentplayer))

(event `DoAIAction`
  (bind _dices (`self.Dices`))
  (bind _output (`|GetArrayItem` (`self.Dices`)))
  ;[1 1 1] Computer turn
  (bind (_result _opponent) (`/Game/Blueprints/Grid/BP_Generator.GetMoveLength` (`self.TileGeneratorRef`) (`self.CurrentPlayer`) (`BlueprintGameplayTagLibrary.GetTagName` (`BlueprintGameplayTagLibrary.MakeLiteralGameplayTag` (struct :`TagName` "Game.PlayerTag.Human")))))
  (if (> _result 1)
    (if (> (`KismetArrayLibrary.Array_Length` _dices) 0) :!label _label_2
      (bind _output_get (set `self.Tokens` (+ (`self.Tokens`) _output)))
      (`KismetSystemLibrary.PrintText` (`|FormatText` "Move token {tokens}" _output))
      (`KismetArrayLibrary.Array_Remove` _dices)
      (if (>= _output_get _result)
        (`self.ComputerMove` :!label _label_3)
        (add `self.OnComputerMoveEnd` (delegate `MoveEnd`))
        (else
          (goto _label_2)))
      (elif (> (`self.Tokens`) 0)
        (goto _label_3)))
    (elif (> (`KismetArrayLibrary.Array_Length` (`self.Dices`)) 0)
      (`self.ApplyDamageAgain`)
      (else
        (`self.NextTurn`)))))

(event `OnFollowPathEnded`
  ;[1 1 1] Computer move
  (set `self.Tokens` 0)
  (`/Game/Blueprints/Grid/BP_Generator.RemoveTags` (`self.TileGeneratorRef`))
  (`self.OnComputerMoveEnd`))

(event `ApplyDamageAgain`
  (bind _output (`|GetArrayItem` (`self.Dices`)))
  ;[1 1 1] Computer turn
  (if (`/Game/Blueprints/Components/Health_System.IsAlive` (`/Game/Blueprints/Player/BP_DefaultHero.Health_System` (stale `DoAIAction` _opponent)))
    (`/Game/Blueprints/Components/Basic_Actions.Damage _Event` (`self.GetComponentByClass` (stale `DoAIAction` _opponent) "/Game/Blueprints/Components/Basic_Actions.Basic_Actions_C") _output :!label _label_4)
    (`KismetSystemLibrary.PrintText` (`|FormatText` "Atak token {token}" _output))
    (add `self.OnTakeAnyDamage` (delegate `ApplyDamege`))
    (`KismetArrayLibrary.Array_Remove` (`self.Dices`))
    (if (> (`KismetArrayLibrary.Array_Length` (`self.Dices`)) 0) :!label _label_5
      (`self.ApplyDamageAgain`)
      (else
        (`KismetSystemLibrary.Delay` 1.0)
        (`self.NextTurn`)))
    (else
      (`self.DoAIAction`))))

(event `MoveEnd`
  ;[1 1 1] Computer turn
  (if (> (`KismetArrayLibrary.Array_Length` (`self.Dices`)) 0)
    (goto _label_4)
    (else
      (`self.NextTurn`))))

(event `ApplyDamege` :!signature `self.OnTakeAnyDamage`
  (params (DamagedActor :type "Actor Object Reference") (Damage :type "Float (single-precision)") (DamageType :type "DamageType Object Reference") (InstigatedBy :type "Controller Object Reference") (DamageCauser :type "Actor Object Reference"))
  ;[1 1 1] Computer turn
  (goto _label_5))

(fn `GetIndex`
  (params (Position :type "Vector2D Structure"))
  (returns (Index :type Integer))
  (return (`KismetMathLibrary.FTrunc` (+ Position_X (* Position_Y (`/Game/Blueprints/Grid/BP_Generator.Columns` (`self.TileGeneratorRef`)))))))

(fn `GetRandomTiles`
  (params (PlayersCount :type Integer))
  (returns (RandomInt :type "Array of Integer"))
  (locals (RandomTileInRange :type Integer) (TryCount :type Integer) (MaxAttemps :type Integer :default 10))
  (bind _returnvalue (- PlayersCount 1))
  (bind (_deltarange_x _deltarange_y) (`KismetMathLibrary.BreakVector2D` (`self.DeltaRange`)))
  (`KismetArrayLibrary.Array_Clear` (`self.RandomInt`))
  (set `local.TryCount` 0)
  (for _ (range (+ _returnvalue 1)) :!label _label
    (bind _output_get (set `local.RandomTileInRange` (`KismetMathLibrary.RandomIntegerInRange` 0 (- (* _deltarange_x _deltarange_y) 1)) :!label _label_2))
    (if (>= (`KismetArrayLibrary.Array_Find` (`self.RandomInt`) _output_get) 0)
      (bind _result (`/Engine/EditorBlueprintResources/StandardMacros.IncrementInt` (`local.TryCount`))
        (:`  `
          (set `local.TryCount` _result)
          (if (> (`local.TryCount`) (`local.MaxAttemps`))
            _
            (else
              (goto _label_2)))))
      (else
        (bind _returnvalue_2 (`KismetArrayLibrary.Array_Add` (`self.RandomInt`) (`local.RandomTileInRange`)))
        (if (< _returnvalue_2 _returnvalue)
          (goto _label)
          (else
            _))))
    (return (`self.RandomInt`))))

(fn `ShowFinalScreen`
  (params (ComputerWon :type Boolean))
  (bind _returnvalue (`GameplayStatics.GetPlayerController` 0))
  (bind _returnvalue_2 (`|CreateWidget` "/Game/Blueprints/UI/WBP_FinalScreen.WBP_FinalScreen_C" _returnvalue))
  (if ComputerWon
    (`/Game/Blueprints/UI/WBP_FinalScreen.OnComputerWin` _returnvalue_2)
    (else
      (`/Game/Blueprints/UI/WBP_FinalScreen.OnPlayerWin` _returnvalue_2)))
  (`UserWidget.AddToViewport` _returnvalue_2 0)
  (set `PlayerController.bShowMouseCursor` true _returnvalue)
  (`WidgetBlueprintLibrary.SetInputMode_UIOnlyEx` null null))

(fn `SpawnActors`
  (params (Indexes :type "Array of Integer (by ref)") (StartPosition :type "Vector2D Structure") (Actors :type "Array of /Game/Blueprints/Player/BP_DefaultHero Object Reference (by ref)") (Rotation :type "Vector Structure") (PawnTag :type Name))
  (bind (_deltarange_x _deltarange_y) (`KismetMathLibrary.BreakVector2D` (`self.DeltaRange`)))
  (for _array_element Indexes
    (bind _returnvalue (mod _array_element (`KismetMathLibrary.FTrunc` _deltarange_y)))
    (bind _index (`self.GetIndex` (`KismetMathLibrary.MakeVector2D` (+ (/ (- _array_element _returnvalue) _deltarange_y) StartPosition_X) (+ _returnvalue StartPosition_Y))))
    (bind _output (`|GetArrayItem` (`/Game/Blueprints/Grid/BP_Generator.Tiles` (`self.TileGeneratorRef`)) _index))
    (bind (_returnvalue_x _returnvalue_y) (`KismetMathLibrary.BreakVector` (`SceneComponent.K2_GetComponentLocation` (`self.GetComponentByClass` _output "/Script/Engine.StaticMeshComponent"))))
    (bind _returnvalue_2 (`|SpawnActorFromClass` "/Game/Blueprints/Player/BP_DefaultHero.BP_DefaultHero_C" (`KismetMathLibrary.MakeTransform` (`KismetMathLibrary.MakeVector` _returnvalue_x _returnvalue_y 126.0) (`KismetMathLibrary.Conv_VectorToRotator` Rotation)) "Undefined" "MultiplyWithRoot" null null))
    (set `/Game/Blueprints/Player/BP_DefaultHero.Tile` _output _returnvalue_2)
    (`KismetArrayLibrary.Array_Add` Actors _returnvalue_2)
    (if (not (== PawnTag "None"))
      (`KismetArrayLibrary.Array_AddUnique` (`Actor.Tags` _returnvalue_2) PawnTag)
      (bind _aswbp_health_bar (cast `/Game/Blueprints/HUD/WBP_HealthBar` (`WidgetComponent.GetWidget` (`/Game/Blueprints/Player/BP_DefaultHero.HealthBar` _returnvalue_2))))
      (set `/Game/Blueprints/HUD/WBP_HealthBar.Health Component Ref` (`self.GetComponentByClass` _returnvalue_2 "/Game/Blueprints/Components/Health_System.Health_System_C") _aswbp_health_bar))))

(fn `UserConstructionScript`)