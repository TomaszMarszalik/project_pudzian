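; Grid-based warrior character that walks tile by tile along a given path, with selection and hover flags.
; FollowPath starts a recursive loop in which a Movement timeline, scaled to per-tile duration, lerps location and yaw, adding a jump arc between tiles of differing height.
; Each step notifies listeners and clears a tile state on the Grid, while animation states reach the AnimBP by message.
; Construction sets mesh, animation class and movement stats.
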(event `self.ReceiveBeginPlay`
  (`self.Set Character anim state` "NewEnumerator0"))

(event `Follow Path`
  (params (Path :type "Array of IntPoint Structure"))
  (if (> (`KismetArrayLibrary.Array_Length` Path) 0)
    (`self.On Character Started Walking` self)
    (set `self.Path` Path)
    (`self.ContinuetoFollow`)))

(event `ContinuetoFollow`
  (bind _movement (`self.Movement`))
  (bind _grid (`self.Grid`))
  (bind _location (.location (`.TileTransform_9_C8B49F424080CB25DC8191A7EE85CF00` (break `/Game/Blueprints/Grid/F_TileData` (`BlueprintMapLibrary.Map_Find` (`/Game/Blueprints/Grid/BP_Grid.Grid Tiles Data` (`self.Grid`)) (`|GetArrayItem` (`self.Path`)))))))
  (bind (_returnvalue_roll _returnvalue_pitch _returnvalue_yaw) (`KismetMathLibrary.BreakRotator` (`KismetMathLibrary.FindLookAtRotation` (.location (`self.Previous Transform`)) _location)))
  (if (> (`KismetArrayLibrary.Array_Length` (`self.Path`)) 0)
    (`self.Set Character anim state` "NewEnumerator1")
    (set `self.Previous Transform` (`self.GetTransform`))
    (set `self.Next Transform` (`KismetMathLibrary.MakeTransform` _location (`KismetMathLibrary.MakeRotator` 0.0 0.0 _returnvalue_yaw)))
    (`TimelineComponent.SetPlayRate` _movement (/ (`TimelineComponent.GetTimelineLength` _movement) (`self.Move Duration per tile`)))
    (bind (_direction _location_alpha _roation_alpha _jump) (`Timeline|Movement` :!via `PlayFromStart`)
      (:`Update`
        (`self.K2_SetActorLocationAndRotation` (+ (`KismetMathLibrary.VLerp` (.location (`self.Previous Transform`)) (.location (`self.Next Transform`)) _location_alpha) (`KismetMathLibrary.MakeVector` 0.0 0.0 (`KismetMathLibrary.SelectFloat` 0.0 _jump (`KismetMathLibrary.NearlyEqual_FloatFloat` (.z (.location (`self.Next Transform`))) (.z (.location (`self.Previous Transform`))) 5.0)))) (`KismetMathLibrary.RLerp` (.rotation (`self.Previous Transform`)) (.rotation (`self.Next Transform`)) _roation_alpha true) false true))
      (:`Finished`
        (`self.On Character Reach New Tile` self (`|GetArrayItem` (`self.Path`)))
        (`/Game/Blueprints/Grid/BP_Grid.removestatetotile` _grid (`.Index_10_EBED7CD648D9AC57BB540D8281F68B1E` (break `/Game/Blueprints/Grid/F_TileData` (`BlueprintMapLibrary.Map_Find` (`/Game/Blueprints/Grid/BP_Grid.Grid Tiles Data` _grid) (`|GetArrayItem` (`self.Path`))))) "NewEnumerator4")
        (`KismetArrayLibrary.Array_Remove` (`self.Path`))
        (`self.ContinuetoFollow`)))
    (else
      (`self.Set Character anim state` "NewEnumerator0")
      (`self.On Character Finnished walking` self))))

(fn `Set Character anim state`
  (params (`Anim State` :type "/Game/Art/Characters/Enum_DebugAnimState Enum" :default "NewEnumerator0"))
  (message `/Game/Art/Characters/BPI_UniAniations.Set Anim State` (`SkeletalMeshComponent.GetAnimInstance` (`self.Skeletal Mesh`)) `Anim State`))

(fn `Set Grid`
  (params (Grid :type "/Game/Blueprints/Grid/BP_Grid Object Reference"))
  (set `self.Grid` Grid))

(fn `Set Is Hovered`
  (params (`Is Hovered` :type Boolean))
  (bind _output_get (set `self.Is Hovered` `Is Hovered`))
  (if _output_get
    _))

(fn `Set is Selected`
  (params (`Is Selected` :type Boolean))
  (bind _output_get (set `self.Is Selected` `Is Selected`))
  (`KismetSystemLibrary.PrintString` (`KismetStringLibrary.Conv_BoolToString` _output_get)))

(fn `UserConstructionScript`
  (bind _skeletal_mesh (`self.Skeletal Mesh`))
  (bind _stats (break `/Game/Blueprints/Characters/F_CharacterData` (`self.Character Data`)))
  (`BlueprintMapLibrary.Map_Add` (`.BasicTokens_18_8B625E0E40F4273FA4F5BCB0E73A6C91` (break `/Game/Blueprints/Characters/F_CharacterData_Stats` _stats)) "speed" 2)
  (bind _structout (setmembers `/Game/Blueprints/Characters/F_CharacterData_Stats` :`StructRef` _stats :`Can move diagonaly` true))
  (`SkeletalMeshComponent.SetSkeletalMeshAsset` _skeletal_mesh "/Game/Art/Characters/Debug_Hero1/SK_Warrior.SK_Warrior")
  (`SkeletalMeshComponent.SetAnimInstanceClass` _skeletal_mesh "/Game/Art/Characters/Debug_Hero1/ABP_WarriorAnimation.ABP_WarriorAnimation_C"))