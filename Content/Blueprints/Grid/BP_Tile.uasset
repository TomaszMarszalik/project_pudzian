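; Clickable grid tile actor that lets the current player move across a square or hexagonal board.
; Initialize picks the mesh for the tile type, attaches to its owner and positions itself from grid coordinates and mesh bounds, staggering alternate hex rows or columns.
; Hovering a move-available tagged tile has BP_Generator highlight the path and stores it on the current player.
; Clicking one sets the player's tile and starts path following.
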(event `self.ReceiveBeginPlay`
  ;[1 1 1] Initiate controller reference
  (bind _asgs_state (cast `/Game/GS_State` (`GameplayStatics.GetGameState`)))
  (set `self.GameStateRef` _asgs_state)
  (bind _asbp_aicontroler (cast `/Game/AI/BP_AIControler` (`AIBlueprintHelperLibrary.GetAIController` (`/Game/GS_State.CurrentPlayer` _asgs_state))))
  (set `self.PlayerControllerRef` _asbp_aicontroler)
  (bind _returnvalue (`GameplayStatics.GetActorOfClass` "/Game/Blueprints/Grid/BP_Generator.BP_Generator_C"))
  (set `self.Grid` (`/Game/Blueprints/Grid/BP_Generator.Tiles` _returnvalue))
  (bind _returnvalue_2 (`GameplayStatics.GetActorOfClass` "/Game/Blueprints/Grid/BP_Generator.BP_Generator_C"))
  (set `self.GridGeneratorRef` _returnvalue_2))

(event `self.ReceiveActorOnClicked`
  (params (ButtonPressed :type "Key Structure"))
  (bind _currentplayer (`/Game/GS_State.CurrentPlayer` (`self.GameStateRef`)))
  ;[1 1 1] Set target location vector
  (if (`KismetArrayLibrary.Array_Contains` (`Actor.Tags` (`ActorComponent.GetOwner` (`self.Tile`))) (`BlueprintGameplayTagLibrary.GetTagName` (`BlueprintGameplayTagLibrary.MakeLiteralGameplayTag` (struct :`TagName` "Grid.Tiles.MoveAvaliable"))))
    (set `/Game/Blueprints/Player/BP_DefaultHero.Tile` self _currentplayer)
    (`/Game/Blueprints/Grid/BP_Generator.BlurAvailableMoveTiles` (`self.GridGeneratorRef`))
    (`/Game/Blueprints/Player/BP_DefaultHero.FollowPath` _currentplayer)))

(event `self.ReceiveActorBeginCursorOver`
  (bind _gridgeneratorref (`self.GridGeneratorRef`))
  (bind _currentplayer (`/Game/GS_State.CurrentPlayer` (`self.GameStateRef`)))
  ;[1 1 1] Focus path
  (if (`KismetArrayLibrary.Array_Contains` (`Actor.Tags` (`ActorComponent.GetOwner` (`self.Tile`))) (`BlueprintGameplayTagLibrary.GetTagName` (`BlueprintGameplayTagLibrary.MakeLiteralGameplayTag` (struct :`TagName` "Grid.Tiles.MoveAvaliable"))))
    (`/Game/Blueprints/Grid/BP_Generator.BlurPathTiles` _gridgeneratorref)
    (bind _actorpath (`/Game/Blueprints/Grid/BP_Generator.Add Tag for Path Tiles` _gridgeneratorref (`/Game/Blueprints/Grid/BP_Tile.Position` (`/Game/Blueprints/Player/BP_DefaultHero.Tile` _currentplayer)) (`self.Position`) false))
    (`/Game/Blueprints/Grid/BP_Generator.FocusPathTiles` _gridgeneratorref)
    (set `/Game/Blueprints/Player/BP_DefaultHero.CurrentFollowPath` _actorpath _currentplayer)
    (else
      (`/Game/Blueprints/Grid/BP_Generator.BlurPathTiles` _gridgeneratorref))))

(fn `CalculateLocation`
  (params (InType :type "/Game/Blueprints/Grid/EGridType Enum" :default "NewEnumerator0"))
  (returns (OutLocation :type "Vector Structure"))
  (bind (_position_x _position_y) (`KismetMathLibrary.BreakVector2D` (`self.Position`)))
  (bind (_position_x_2 _position_y_2) (`KismetMathLibrary.BreakVector2D` (`self.Position`)))
  (bind (_position_x_3 _position_y_3) (`KismetMathLibrary.BreakVector2D` (`self.Position`)))
  (bind _y (.y (`.BoxExtent` (`KismetSystemLibrary.GetComponentBounds` (`self.Tile`)))))
  (bind _x (.x (`.BoxExtent` (`KismetSystemLibrary.GetComponentBounds` (`self.Tile`)))))
  (bind _returnvalue (* _x 2.0 _position_y_2))
  (bind _returnvalue_2 (* _y 2.0 _position_x))
  (return (select `/Game/Blueprints/Grid/EGridType` InType :`NewEnumerator0` (`KismetMathLibrary.MakeVector` (* (.x (`.BoxExtent` (`KismetSystemLibrary.GetComponentBounds` (`self.Tile`)))) _position_x_3) (* (.y (`.BoxExtent` (`KismetSystemLibrary.GetComponentBounds` (`self.Tile`)))) _position_y_3)) :`NewEnumerator1` (`KismetMathLibrary.MakeVector` (`KismetMathLibrary.SelectFloat` _returnvalue_2 (+ _returnvalue_2 _y) (== (mod (`KismetMathLibrary.FTrunc` _position_y) 2) 0)) (* (.x (`.BoxExtent` (`KismetSystemLibrary.GetComponentBounds` (`self.Tile`)))) 2.0 _position_y (/ 3.0 4.0))) :`NewEnumerator2` (`KismetMathLibrary.MakeVector` (* (.y (`.BoxExtent` (`KismetSystemLibrary.GetComponentBounds` (`self.Tile`)))) 2.0 _position_x_2 (/ 3.0 4.0)) (`KismetMathLibrary.SelectFloat` _returnvalue (+ _returnvalue _x) (== (mod (`KismetMathLibrary.FTrunc` _position_x_2) 2) 0))))))

(fn `Initialize`
  (params (InType :type "/Game/Blueprints/Grid/EGridType Enum" :default "NewEnumerator0"))
  (bind _returnvalue (`self.GetOwner`))
  (`/Engine/EditorBlueprintResources/StandardMacros.IsValid` _returnvalue
    (:`Is Valid`
      (`self.SetMesh` InType)
      (`self.K2_AttachToActor` _returnvalue "None" "SnapToTarget" "KeepWorld" "KeepRelative" false)
      (bind _outlocation (`self.CalculateLocation` (`local.InType`)))
      (`self.K2_SetActorRelativeLocation` _outlocation))))

(fn `SetMesh`
  (params (InType :type "/Game/Blueprints/Grid/EGridType Enum" :default "NewEnumerator0"))
  (`StaticMeshComponent.SetStaticMesh` (`self.Tile`) (select `/Game/Blueprints/Grid/EGridType` InType :`NewEnumerator0` "/Engine/BasicShapes/Plane.Plane" :`NewEnumerator1` "/Game/Meshes/Hexagon_PP_3C_Top.Hexagon_PP_3C_Top" :`NewEnumerator2` "/Game/Meshes/Hexagon_FF_3C_Top.Hexagon_FF_3C_Top" :!type "StaticMesh Object Reference")))

(fn `UserConstructionScript`)