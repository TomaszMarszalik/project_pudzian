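; BP_Generator spawns the BP_Tile grid and drives movement targeting for turn-based human and computer heroes.
; GridRangeFinder supplies hex ranges and paths, which are stored as gameplay-tag names on tiles and shown through material swaps.
; Computer turns path toward the nearest human within move range, excluding occupied tiles, and assign the last path tile to the hero.
; It also outlines opponents within path distance and includes debug test events.
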(event Custom|Test%20Show%20Available%20Move%20Tiles
  (bind _returnvalue (Math|Vector2D|MakeVector2D 7.0 8.0))
  (bind _tiles (Variables|Default|GetTiles))
  (bind _output (Utilities|Array|Get(acopy) _tiles))
  (bind _returnvalue_2 (Transformation|GetActorLocation _output))
  ;[1 1 1] Test add tag available move and focus tiles
  (CallFunction|GetTileIndex _returnvalue)
  (bind _returnvalue_3 (Actor|GetActorOfClass "/Game/AI/EQS/EQS_Testing_Pawn.EQS_Testing_Pawn_C"))
  (Transformation|SetActorLocation _returnvalue_3 (Math|Vector|MakeVector (.x _returnvalue_2) (.y _returnvalue_2) (.z (Transformation|GetActorLocation _returnvalue_3))) false false)
  (CallFunction|AddTagforAvaliableMoveTilesinRange _returnvalue (Utilities|Array|MakeArray _returnvalue) 3)
  (CallFunction|FocusAvailableMoveTiles))

(event Custom|FocusPathTiles
  ;[1 1 1] Set material for show path
  (bind _outactors (Actor|GetAllActorsOfClasswithTag "/Game/Blueprints/Grid/BP_Tile.BP_Tile_C" (GameplayTags|GetTagName (GameplayTags|MakeLiteralGameplayTag "(TagName=\"Grid.Tiles.PathAvailable\")"))))
  (for _array_element _outactors
    (Rendering|Material|SetMaterial (Variables|/Game/Blueprints/Grid/BP_Tile.BP_Tile_C|GetTile _array_element) 0 (Variables|Default|GetPathMaterial))))

(event Custom|Test%20Remove%20Overlay%20Material
  ;[1 1 1] Test Remove Overlay material
  (bind _outactors (Actor|GetAllActorsOfClasswithTag "/Game/Blueprints/Player/BP_DefaultHero.BP_DefaultHero_C" (GameplayTags|GetTagName (GameplayTags|MakeLiteralGameplayTag "(TagName=\"Game.PlayerTag.Human\")"))))
  (for _array_element _outactors
    (Rendering|Material|SetOverlayMaterial (Variables|/Script/Engine.Character|GetMesh _array_element) 0 :!class /Script/Engine.MeshComponent)))

(event Custom|Test%20move%20to%20near%20Player
  ;[1 1 1] Test path to player
  (bind _outactors (Actor|GetAllActorsOfClasswithTag "/Game/Blueprints/Player/BP_DefaultHero.BP_DefaultHero_C" (GameplayTags|GetTagName (GameplayTags|MakeLiteralGameplayTag "(TagName=\"Game.PlayerTag.Computer\")"))))
  (bind _player (CallFunction|GetNearPlayer (Variables|/Game/Blueprints/Grid/BP_Tile.BP_Tile_C|GetPosition (Variables|/Game/Blueprints/Player/BP_DefaultHero.BP_DefaultHero_C|GetTile (Utilities|Array|Get(acopy) _outactors)))))
  (bind _actorpath (CallFunction|AddTagforPathTiles (Variables|/Game/Blueprints/Grid/BP_Tile.BP_Tile_C|GetPosition (Variables|/Game/Blueprints/Player/BP_DefaultHero.BP_DefaultHero_C|GetTile (Utilities|Array|Get(acopy) _outactors))) (Variables|/Game/Blueprints/Grid/BP_Tile.BP_Tile_C|GetPosition (Variables|/Game/Blueprints/Player/BP_DefaultHero.BP_DefaultHero_C|GetTile _player)) true))
  (bind _output_get (Variables|/Game/Blueprints/Player/BP_DefaultHero.BP_DefaultHero_C|SetCurrentFollowPath (Utilities|Array|Get(acopy) _outactors) _actorpath))
  (Variables|/Game/Blueprints/Player/BP_DefaultHero.BP_DefaultHero_C|SetTile (Utilities|Array|Get(acopy) _outactors) (Utilities|Array|Get(acopy) _output_get (Utilities|Array|LastIndex _output_get)))
  (Default|FollowPath (Utilities|Array|Get(acopy) _outactors)))

(event Custom|HumanPlayerFocusMovement
  (params (MaxDistance :type Integer))
  ;[1 1 1] Human move range
  (CallFunction|BlurAvailableMoveTiles)
  (bind _array (CallFunction|GetExcludeTilesVector2D))
  (CallFunction|AddTagforAvaliableMoveTilesinRange (Variables|/Game/Blueprints/Grid/BP_Tile.BP_Tile_C|GetPosition (Variables|/Game/Blueprints/Player/BP_DefaultHero.BP_DefaultHero_C|GetTile (Variables|/Game/GS_State.GS_State_C|GetCurrentPlayer (Variables|Default|GetGameStateRef)))) _array MaxDistance)
  (CallFunction|FocusAvailableMoveTiles))

(event Custom|Test%20Path%20to%20Near%20Player
  ;[1 1 1] Test path to player
  (bind _outactors (Actor|GetAllActorsOfClasswithTag "/Game/Blueprints/Player/BP_DefaultHero.BP_DefaultHero_C" (GameplayTags|GetTagName (GameplayTags|MakeLiteralGameplayTag "(TagName=\"Game.PlayerTag.Computer\")"))))
  (bind _player (CallFunction|GetNearPlayer (Variables|/Game/Blueprints/Grid/BP_Tile.BP_Tile_C|GetPosition (Variables|/Game/Blueprints/Player/BP_DefaultHero.BP_DefaultHero_C|GetTile (Utilities|Array|Get(acopy) _outactors)))))
  (CallFunction|BlurPathTiles)
  (CallFunction|AddTagforPathTiles (Variables|/Game/Blueprints/Grid/BP_Tile.BP_Tile_C|GetPosition (Variables|/Game/Blueprints/Player/BP_DefaultHero.BP_DefaultHero_C|GetTile (Utilities|Array|Get(acopy) _outactors))) (Variables|/Game/Blueprints/Grid/BP_Tile.BP_Tile_C|GetPosition (Variables|/Game/Blueprints/Player/BP_DefaultHero.BP_DefaultHero_C|GetTile _player)) true)
  (CallFunction|FocusPathTiles))

(event Custom|ComputerPathWay
  (params (MoveRange :type Integer))
  ;[1 1 1] Computer Move path
  (bind _array (CallFunction|GetExcludeTilesVector2D))
  (CallFunction|AddTagforAvaliableMoveTilesinRange (Variables|/Game/Blueprints/Grid/BP_Tile.BP_Tile_C|GetPosition (Variables|/Game/Blueprints/Player/BP_DefaultHero.BP_DefaultHero_C|GetTile (Variables|/Game/GS_State.GS_State_C|GetCurrentPlayer (Variables|Default|GetGameStateRef)))) _array MoveRange)
  (bind _player (CallFunction|GetNearPlayer (Variables|/Game/Blueprints/Grid/BP_Tile.BP_Tile_C|GetPosition (Variables|/Game/Blueprints/Player/BP_DefaultHero.BP_DefaultHero_C|GetTile (Variables|/Game/GS_State.GS_State_C|GetCurrentPlayer (Variables|Default|GetGameStateRef))))))
  (bind _actorpath (CallFunction|AddTagforPathTiles (Variables|/Game/Blueprints/Grid/BP_Tile.BP_Tile_C|GetPosition (Variables|/Game/Blueprints/Player/BP_DefaultHero.BP_DefaultHero_C|GetTile (Variables|/Game/GS_State.GS_State_C|GetCurrentPlayer (Variables|Default|GetGameStateRef)))) (Variables|/Game/Blueprints/Grid/BP_Tile.BP_Tile_C|GetPosition (Variables|/Game/Blueprints/Player/BP_DefaultHero.BP_DefaultHero_C|GetTile _player)) true))
  (bind _output_get (Variables|/Game/Blueprints/Player/BP_DefaultHero.BP_DefaultHero_C|SetCurrentFollowPath (Variables|/Game/GS_State.GS_State_C|GetCurrentPlayer (Variables|Default|GetGameStateRef)) _actorpath))
  (Variables|/Game/Blueprints/Player/BP_DefaultHero.BP_DefaultHero_C|SetTile (Variables|/Game/GS_State.GS_State_C|GetCurrentPlayer (Variables|Default|GetGameStateRef)) (Utilities|Array|Get(acopy) _output_get (Utilities|Array|LastIndex _output_get))))

(event Custom|CleanUp
  (CallFunction|BlurPathTiles)
  (CallFunction|RemovePathTags)
  (CallFunction|BlurAvailableMoveTiles)
  (CallFunction|RemoveMoveTags))

(event Custom|CleanUpTags
  (CallFunction|RemovePathTags)
  (CallFunction|RemoveMoveTags))

(event Custom|BlurAvailableMoveTiles
  (bind _returnvalue (GameplayTags|MakeLiteralGameplayTag "(TagName=\"Grid.Tiles.MoveAvaliable\")"))
  (bind _returnvalue_2 (GameplayTags|GetTagName _returnvalue))
  ;[1 1 1] Set material for hide avaliable move
  (bind _outactors (Actor|GetAllActorsOfClasswithTag "/Game/Blueprints/Grid/BP_Tile.BP_Tile_C" _returnvalue_2))
  (for _array_element _outactors
    (Rendering|Material|SetMaterial (Actor|GetComponentbyClass _array_element "/Script/Engine.StaticMeshComponent") 0 "/Game/Materials/M_None.M_None")
    (Utilities|Array|RemoveIndex (Variables|/Script/Engine.Actor|GetTags _array_element) (Utilities|Array|FindItem (Variables|/Script/Engine.Actor|GetTags _array_element) _returnvalue_2))))

(event Custom|FocusAvailableMoveTiles
  ;[1 1 1] Set material for show available move
  (bind _outactors (Actor|GetAllActorsOfClasswithTag "/Game/Blueprints/Grid/BP_Tile.BP_Tile_C" (GameplayTags|GetTagName (GameplayTags|MakeLiteralGameplayTag "(TagName=\"Grid.Tiles.MoveAvaliable\")"))))
  (for _array_element _outactors
    (Rendering|Material|SetMaterial (Actor|GetComponentbyClass _array_element "/Script/Engine.StaticMeshComponent") 0 "/Game/Materials/M_AvaliableMove.M_AvaliableMove")))

(event Custom|RemoveMoveTags
  ;[1 1 1] Remove available mov tags
  (bind _outactors (Actor|GetAllActorsOfClasswithTag "/Game/Blueprints/Grid/BP_Tile.BP_Tile_C" (GameplayTags|GetTagName (GameplayTags|MakeLiteralGameplayTag "(TagName=\"Grid.Tiles.MoveAvaliable\")"))))
  (for _array_element _outactors
    (Utilities|Array|RemoveIndex _outactors)))

(event Custom|RemovePathTags
  ;[1 1 1] Remove path tags
  (bind _outactors (Actor|GetAllActorsOfClasswithTag "/Game/Blueprints/Grid/BP_Tile.BP_Tile_C" (GameplayTags|GetTagName (GameplayTags|MakeLiteralGameplayTag "(TagName=\"Grid.Tiles.PathAvailable\")"))))
  (for _array_element _outactors
    (Utilities|Array|RemoveIndex _outactors)))

(event Custom|BlurPathTiles
  (bind _returnvalue (GameplayTags|MakeLiteralGameplayTag "(TagName=\"Grid.Tiles.PathAvailable\")"))
  (bind _returnvalue_2 (GameplayTags|GetTagName _returnvalue))
  ;[1 1 1] Set material for hide path
  (if (CallFunction|IsHuman)
    (bind _outactors (Actor|GetAllActorsOfClasswithTag "/Game/Blueprints/Grid/BP_Tile.BP_Tile_C" _returnvalue_2))
    (for _array_element _outactors
      (if (>= (Utilities|Array|FindItem (Variables|/Script/Engine.Actor|GetTags _array_element) _returnvalue_2) 0)
        (Utilities|Array|RemoveIndex (Variables|/Script/Engine.Actor|GetTags _array_element) (Utilities|Array|FindItem (Variables|/Script/Engine.Actor|GetTags _array_element) _returnvalue_2))
        (if (Actor|ActorHasTag (Components|GetOwner (Variables|/Game/Blueprints/Grid/BP_Tile.BP_Tile_C|GetTile _array_element)) (GameplayTags|GetTagName (GameplayTags|MakeLiteralGameplayTag "(TagName=\"Grid.Tiles.MoveAvaliable\")")))
          (if (CallFunction|IsHuman)
            (Rendering|Material|SetMaterial (Variables|/Game/Blueprints/Grid/BP_Tile.BP_Tile_C|GetTile _array_element) 0 (Variables|Default|GetAvaliableMoveMaterial))
            (else
              (Rendering|Material|SetMaterial (Variables|/Game/Blueprints/Grid/BP_Tile.BP_Tile_C|GetTile _array_element) 0 (Variables|Default|GetGridBaseMaterial) :!label _label)))
          (else
            (goto _label)))))))

(event Custom|Test%20remove%20path%20tag
  ;[1 1 1] Test remove tag avaliable move and blur tiles
  (Actor|GetActorOfClass "BP_Generator_C")
  (CallFunction|BlurPathTiles))

(event Custom|Test%20Find%20%20Nearest%20Player
  ;[1 1 1] Fnd nearest player
  (bind _outactors (Actor|GetAllActorsOfClasswithTag "/Game/Blueprints/Player/BP_DefaultHero.BP_DefaultHero_C" (GameplayTags|GetTagName (GameplayTags|MakeLiteralGameplayTag "(TagName=\"Game.PlayerTag.Computer\")"))))
  (bind _player (CallFunction|GetNearPlayer (Variables|/Game/Blueprints/Grid/BP_Tile.BP_Tile_C|GetPosition (Variables|/Game/Blueprints/Player/BP_DefaultHero.BP_DefaultHero_C|GetTile (Utilities|Array|Get(acopy) _outactors)))))
  (Utilities|IsValid _player
    (:Is%20Valid
      (Rendering|Material|SetOverlayMaterial (Variables|/Script/Engine.Character|GetMesh _player) "/Game/Materials/M_Outline.M_Outline" :!class /Script/Engine.MeshComponent))))

(event Custom|Test%20Remove%20Available%20Move%20Tag
  ;[1 1 1] Test remove tag avaliable move and blur tiles
  (bind _returnvalue (Actor|GetActorOfClass "BP_Generator_C"))
  (CallFunction|BlurAvailableMoveTiles _returnvalue))

(event EventBeginPlay
  (bind _returnvalue (Actor|GetActorOfClass "/Game/GS_State.GS_State_C"))
  (Variables|Default|SetGameStateRef _returnvalue))

(event Input|KeyboardEvents|DebugKeyB
  (params (Key :type Key%20Structure :default "None") (ActionValue :type Input%20Action%20Value%20Structure))
  ;[1 1 1] Test path to player
  (:Pressed
    (bind _outactors (Actor|GetAllActorsOfClasswithTag "/Game/Blueprints/Player/BP_DefaultHero.BP_DefaultHero_C" (GameplayTags|GetTagName (GameplayTags|MakeLiteralGameplayTag "(TagName=\"Game.PlayerTag.Computer\")"))))
    (bind _player (CallFunction|GetNearPlayer (Variables|/Game/Blueprints/Grid/BP_Tile.BP_Tile_C|GetPosition (Variables|/Game/Blueprints/Player/BP_DefaultHero.BP_DefaultHero_C|GetTile (Utilities|Array|Get(acopy) _outactors)))))
    (bind _actorpath (CallFunction|AddTagforPathTiles (Variables|/Game/Blueprints/Grid/BP_Tile.BP_Tile_C|GetPosition (Variables|/Game/Blueprints/Player/BP_DefaultHero.BP_DefaultHero_C|GetTile (Utilities|Array|Get(acopy) _outactors))) (Variables|/Game/Blueprints/Grid/BP_Tile.BP_Tile_C|GetPosition (Variables|/Game/Blueprints/Player/BP_DefaultHero.BP_DefaultHero_C|GetTile _player)) true))
    (bind _output_get (Variables|/Game/Blueprints/Player/BP_DefaultHero.BP_DefaultHero_C|SetCurrentFollowPath (Utilities|Array|Get(acopy) _outactors) _actorpath))
    (Variables|/Game/Blueprints/Player/BP_DefaultHero.BP_DefaultHero_C|SetTile (Utilities|Array|Get(acopy) _outactors) (Utilities|Array|Get(acopy) _output_get (Utilities|Array|LastIndex _output_get)))
    (Default|FollowPath (Utilities|Array|Get(acopy) _outactors))))

(fn ConstructionScript)

(fn InitializeTiles
  (CallFunction|ClearTiles)
  (for _index (range 0 (- (Variables|Default|GetRows) 1))
    (for _index_2 (range 0 (- (Variables|Default|GetColumns) 1))
      (bind _returnvalue (Game|SpawnActorfromClass "/Game/Blueprints/Grid/BP_Tile.BP_Tile_C" (Math|Transform|MakeTransform (Transformation|GetActorLocation) (Transformation|GetActorRotation)) "AlwaysSpawn" "MultiplyWithRoot" self (Math|Vector2D|MakeVector2D (Math|Conversions|ToFloat(Integer) _index_2) (Math|Conversions|ToFloat(Integer) _index)) 0))
      (Default|Initialize _returnvalue (Variables|Default|GetType))
      (Utilities|Array|Add (Variables|Default|GetTiles) _returnvalue))))

(fn ClearTiles
  (bind _tiles (Variables|Default|GetTiles))
  (if (>= (Utilities|Array|Length (Variables|Default|GetTiles)) 0)
    (for _array_element _tiles
      (Actor|DestroyActor _array_element))
    (Utilities|Array|Clear _tiles)))

(fn GetTileIndex
  (params (Position :type Vector%202D%20Structure))
  (return (Math|Float|Truncate (+ (.x Position) (* (.y Position) (Variables|Default|GetColumns))))))

(fn AddTagforAvaliableMoveTilesinRange
  (params (Position :type Vector%202D%20Structure) (Exclude :type Array%20of%20Vector%202D%20Structures) (Range :type Integer))
  (CallFunction|RemoveMoveTags)
  (bind _returnvalue (Class|GridRangeFinderComponent|GetRangeTilesPositions (Variables|Default|GetGridRangeFinder) Position Range "(X=5.000000,Y=2.000000)" "(X=20.000000,Y=11.000000)" Exclude))
  (for _array_element _returnvalue
    (bind _index (CallFunction|GetTileIndex _array_element))
    (Utilities|Array|AddUnique (Variables|/Script/Engine.Actor|GetTags (Utilities|Array|Get(acopy) (Variables|Default|GetTiles) _index)) (GameplayTags|GetTagName (GameplayTags|MakeLiteralGameplayTag "(TagName=\"Grid.Tiles.MoveAvaliable\")")))))

(fn AddTagforPathTiles
  (params (Start :type Vector%202D%20Structure) (Target :type Vector%202D%20Structure) (WithoutContains :type Boolean))
  (if WithoutContains
    _
    (else
      (Utilities|Array|Clear (LocalVariables|GetTargetActorPath))
      (bind _positions (CallFunction|GetPositionsfromTaggedAvalibleMoveTiles))))
  (bind _returnvalue (Class|GridRangeFinderComponent|PathGrid (Variables|Default|GetGridRangeFinder) Start Target _positions))
  (Utilities|Array|Reverse _returnvalue)
  (bind _array_element (Utilities|Array|ForEachLoopwithBreak _returnvalue :!label _label)
    (:LoopBody
      (bind _index (CallFunction|GetTileIndex _array_element))
      (if (Actor|ActorHasTag (Components|GetOwner (Variables|/Game/Blueprints/Grid/BP_Tile.BP_Tile_C|GetTile (Utilities|Array|Get(acopy) (Variables|Default|GetTiles) _index))) (GameplayTags|GetTagName (GameplayTags|MakeLiteralGameplayTag "(TagName=\"Grid.Tiles.MoveAvaliable\")")))
        (Utilities|Array|AddUnique (Variables|/Script/Engine.Actor|GetTags (Components|GetOwner (Variables|/Game/Blueprints/Grid/BP_Tile.BP_Tile_C|GetTile (Utilities|Array|Get(acopy) (Variables|Default|GetTiles) _index)))) (GameplayTags|GetTagName (GameplayTags|MakeLiteralGameplayTag "(TagName=\"Grid.Tiles.PathAvailable\")")))
        (Utilities|Array|Add (LocalVariables|GetTargetActorPath) (Utilities|Array|Get(acopy) (Variables|Default|GetTiles) _index))
        (else
          (goto _label Break))))
    (:Completed
      (return (LocalVariables|GetTargetActorPath)))))

(fn GetPositionsfromTaggedAvalibleMoveTiles
  (Utilities|Array|Clear (LocalVariables|GetAvailableTiles))
  (bind _outactors (Actor|GetAllActorsOfClasswithTag "/Game/Blueprints/Grid/BP_Tile.BP_Tile_C" (GameplayTags|GetTagName (GameplayTags|MakeLiteralGameplayTag "(TagName=\"Grid.Tiles.MoveAvaliable\")"))))
  (for _array_element _outactors
    (Utilities|Array|Add (LocalVariables|GetAvailableTiles) (Variables|/Game/Blueprints/Grid/BP_Tile.BP_Tile_C|GetPosition _array_element)))
  (return (LocalVariables|GetAvailableTiles)))

(fn GetExcludeTilesVector2D
  (bind _outactors (Actor|GetAllActorsOfClass "/Game/Blueprints/Player/BP_DefaultHero.BP_DefaultHero_C"))
  (Utilities|Array|Clear (LocalVariables|GetFilterHex))
  (for _array_element _outactors
    (Utilities|IsValid (Variables|/Game/Blueprints/Player/BP_DefaultHero.BP_DefaultHero_C|GetTile _array_element)
      (:Is%20Valid
        (Utilities|Array|Add (LocalVariables|GetFilterHex) (Variables|/Game/Blueprints/Grid/BP_Tile.BP_Tile_C|GetPosition (Variables|/Game/Blueprints/Player/BP_DefaultHero.BP_DefaultHero_C|GetTile _array_element))))))
  (return (LocalVariables|GetFilterHex)))

(fn GetNearPlayer
  (params (Position :type Vector%202D%20Structure))
  (LocalVariables|SetFindDistance false)
  (bind _outactors (Actor|GetAllActorsOfClasswithTag "/Game/Blueprints/Player/BP_DefaultHero.BP_DefaultHero_C" (GameplayTags|GetTagName (GameplayTags|MakeLiteralGameplayTag "(TagName=\"Game.PlayerTag.Human\")"))))
  (bind _index (CallFunction|GetTileIndex Position))
  (for _array_element _outactors
    (if (LocalVariables|GetFindDistance)
      (if (< (Transformation|GetDistanceTo (Utilities|Array|Get(acopy) (Variables|Default|GetTiles) _index) _array_element) (LocalVariables|GetDistance))
        (LocalVariables|SetNearPlayer _array_element :!label _label)
        (LocalVariables|SetDistance (Transformation|GetDistanceTo (Utilities|Array|Get(acopy) (Variables|Default|GetTiles) _index) _array_element))
        (LocalVariables|SetFindDistance true))
      (else
        (goto _label))))
  (return (LocalVariables|GetNearPlayer)))

(fn GetOpponentinRange
  (params (Distance :type Integer) (PlayerTag :type Name))
  (Utilities|Array|Clear (Variables|Default|GetRangeOpponents))
  (bind _outactors (Actor|GetAllActorsOfClasswithTag "/Game/Blueprints/Player/BP_DefaultHero.BP_DefaultHero_C" PlayerTag))
  (for _array_element _outactors
    (bind _returnvalue (Class|GridRangeFinderComponent|PathGrid (Variables|Default|GetGridRangeFinder) (Variables|/Game/Blueprints/Grid/BP_Tile.BP_Tile_C|GetPosition (Variables|/Game/Blueprints/Player/BP_DefaultHero.BP_DefaultHero_C|GetTile (Variables|/Game/GS_State.GS_State_C|GetCurrentPlayer (Variables|Default|GetGameStateRef)))) (Variables|/Game/Blueprints/Grid/BP_Tile.BP_Tile_C|GetPosition (Variables|/Game/Blueprints/Player/BP_DefaultHero.BP_DefaultHero_C|GetTile _array_element)) (Utilities|Array|MakeArray)))
    (if (<= (Utilities|Array|Length _returnvalue) Distance)
      (Rendering|Material|SetOverlayMaterial (Variables|/Script/Engine.Character|GetMesh _array_element) "/Game/Materials/M_Outline.M_Outline" :!class /Script/Engine.MeshComponent)
      (Utilities|Array|Add (Variables|Default|GetRangeOpponents) _array_element)))
  (return (Variables|Default|GetRangeOpponents)))

(fn RemoveTags
  (CallFunction|RemovePathTags2)
  (CallFunction|RemoveMoveTags2))

(fn RemovePathTags2
  (bind _outactors (Actor|GetAllActorsOfClasswithTag "/Game/Blueprints/Grid/BP_Tile.BP_Tile_C" (GameplayTags|GetTagName (GameplayTags|MakeLiteralGameplayTag "(TagName=\"Grid.Tiles.PathAvailable\")"))))
  (for _array_element _outactors
    (if (>= (Utilities|Array|FindItem (Variables|/Script/Engine.Actor|GetTags _array_element) (GameplayTags|GetTagName (GameplayTags|MakeLiteralGameplayTag "(TagName=\"Grid.Tiles.PathAvailable\")"))) 0)
      (Utilities|Array|RemoveIndex (Variables|/Script/Engine.Actor|GetTags _array_element) (Utilities|Array|FindItem (Variables|/Script/Engine.Actor|GetTags _array_element) (GameplayTags|GetTagName (GameplayTags|MakeLiteralGameplayTag "(TagName=\"Grid.Tiles.PathAvailable\")"))))))
  (return))

(fn RemoveMoveTags2
  (bind _outactors (Actor|GetAllActorsOfClasswithTag "/Game/Blueprints/Grid/BP_Tile.BP_Tile_C" (GameplayTags|GetTagName (GameplayTags|MakeLiteralGameplayTag "(TagName=\"Grid.Tiles.MoveAvaliable\")"))))
  (for _array_element _outactors
    (if (>= (Utilities|Array|FindItem (Variables|/Script/Engine.Actor|GetTags _array_element) (GameplayTags|GetTagName (GameplayTags|MakeLiteralGameplayTag "(TagName=\"Grid.Tiles.MoveAvaliable\")"))) 0)
      (Utilities|Array|RemoveIndex (Variables|/Script/Engine.Actor|GetTags _array_element) (Utilities|Array|FindItem (Variables|/Script/Engine.Actor|GetTags _array_element) (GameplayTags|GetTagName (GameplayTags|MakeLiteralGameplayTag "(TagName=\"Grid.Tiles.MoveAvaliable\")"))))))
  (return))

(fn IsHuman
  (return (Utilities|Array|ContainsItem (Variables|/Script/Engine.Actor|GetTags (Variables|/Game/GS_State.GS_State_C|GetCurrentPlayer (Variables|Default|GetGameStateRef))) (GameplayTags|GetTagName (GameplayTags|MakeLiteralGameplayTag "(TagName=\"Game.PlayerTag.Human\")")))))

(fn IsComputer
  (return (Utilities|Array|ContainsItem (Variables|/Script/Engine.Actor|GetTags (Variables|/Game/GS_State.GS_State_C|GetCurrentPlayer (Variables|Default|GetGameStateRef))) (GameplayTags|GetTagName (GameplayTags|MakeLiteralGameplayTag "(TagName=\"Game.PlayerTag.Human\")")))))