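; Grid tile renderer actor that draws tiles as instances of one configurable mesh, colored by either tile type or tile state.
; A parallel index array maps each tile to its instance, so adding a tile replaces its existing one.
; Color and fill opacity reach the material through per-instance custom data.
; In state mode a fixed priority order picks the color, and tiles without a matching state get zero fill opacity.
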(fn `Add Instance`
  (params (InstanceTransform :type "Transform Structure (by ref)") (Index :type "IntPoint Structure (by ref)") (States :type "Array of /Game/Blueprints/Grid/Enum_TileStates Enum") (Types :type "/Game/Blueprints/Grid/Obstacles/Enum_TileTypes Enum" :default "NewEnumerator0"))
  (locals (NewLocalVar :type Integer :default 0))
  (bind _instancedstaticmesh (`self.InstancedStaticMesh`))
  (bind _i (`self.I`))
  (`self.RemoveInstaces` Index)
  (`InstancedStaticMeshComponent.AddInstance` (`self.InstancedStaticMesh`) InstanceTransform false)
  (bind _returnvalue (`KismetArrayLibrary.Array_Add` (`self.Instace Indexs`) Index))
  (set `self.I` _returnvalue)
  (bind (_color _fill_opacity) (`self.Get Color Of Tile` States Types))
  (bind (_r _g _b) (`KismetMathLibrary.BreakColor` _color))
  (`InstancedStaticMeshComponent.SetCustomDataValue` _instancedstaticmesh _i 0 _r false)
  (`InstancedStaticMeshComponent.SetCustomDataValue` _instancedstaticmesh _i 1 _g false)
  (`InstancedStaticMeshComponent.SetCustomDataValue` _instancedstaticmesh _i 2 _b false)
  (`InstancedStaticMeshComponent.SetCustomDataValue` _instancedstaticmesh _i 3 _fill_opacity false))

(fn `ClearInst`
  (`InstancedStaticMeshComponent.ClearInstances` (`self.InstancedStaticMesh`))
  (`KismetArrayLibrary.Array_Clear` (`self.Instace Indexs`)))

(fn `Get Color Of Tile`
  (params (States :type "Array of /Game/Blueprints/Grid/Enum_TileStates Enum") (Types :type "/Game/Blueprints/Grid/Obstacles/Enum_TileTypes Enum" :default "NewEnumerator0"))
  (returns (color :type "LinearColor Structure") (`Fill Opacity` :type "Float (double-precision)"))
  (if (`self.Generate for Types`)
    (return (select `/Game/Blueprints/Grid/Obstacles/Enum_TileTypes` Types :`NewEnumerator0` (struct :`R` 0.028101 :`G` 0.135417 :`A` 1.0) :`NewEnumerator1` (struct :`A` 1.0) :`NewEnumerator2` (struct :`R` 0.255208 :`A` 1.0) :`NewEnumerator6` (struct :`G` 0.101209 :`B` 0.1875 :`A` 1.0) :`NewEnumerator11` (struct :`R` 0.28125 :`G` 0.271956 :`B` 0.155273 :`A` 1.0) :!type "LinearColor Structure") 1.0)
    (elif (== (`KismetArrayLibrary.Array_Length` States) 0)
      (return (struct :`A` 1.0) 0.0)
      (else
        (for _array_element (`|MakeArray` "NewEnumerator6" "NewEnumerator5" "NewEnumerator2" "NewEnumerator1" "NewEnumerator4" "NewEnumerator3" :!type "/Game/Blueprints/Grid/Enum_TileStates Enum")
          (if (`KismetArrayLibrary.Array_Contains` (`local.States`) _array_element)
            (return (select `/Game/Blueprints/Grid/Enum_TileStates` _array_element :`NewEnumerator0` (struct :`A` 1.0) :`NewEnumerator1` (struct :`R` 1.0 :`G` 0.911714 :`A` 1.0) :`NewEnumerator2` (struct :`R` 0.065589 :`G` 1.0 :`A` 1.0) :`NewEnumerator3` (struct :`G` 0.082772 :`B` 0.479167 :`A` 1.0) :`NewEnumerator4` (struct :`R` 0.339199 :`B` 1.0 :`A` 1.0) :`NewEnumerator5` (struct :`R` 0.723055 :`B` 0.005605 :`A` 1.0) :`NewEnumerator6` (struct :`G` 0.881135 :`B` 0.927083 :`A` 1.0) :!type "LinearColor Structure") 0.2)))
        (return (struct :`A` 1.0) 0.0)))))

(fn `InitializeGridInst`
  (params (Mesh :type "StaticMesh Object Reference") (Material :type "MaterialInterface Object Reference") (Collision :type "ECollisionEnabled Enum" :default "NoCollision") (`Generate for Types` :type Boolean))
  (bind _instancedstaticmesh (`self.InstancedStaticMesh`))
  (`StaticMeshComponent.SetStaticMesh` _instancedstaticmesh Mesh)
  (`PrimitiveComponent.SetMaterial` _instancedstaticmesh 0 Material)
  (set `self.Generate for Types` `Generate for Types`)
  (`PrimitiveComponent.SetCollisionEnabled` _instancedstaticmesh Collision))

(fn `RemoveInstaces`
  (params (Index :type "IntPoint Structure (by ref)"))
  (bind _instace_indexs (`self.Instace Indexs`))
  (if (`KismetArrayLibrary.Array_Contains` _instace_indexs Index)
    (`InstancedStaticMeshComponent.RemoveInstance` (`self.InstancedStaticMesh`) (`KismetArrayLibrary.Array_Find` _instace_indexs Index))
    (`KismetArrayLibrary.Array_RemoveItem` _instace_indexs Index)))

(fn `UserConstructionScript`)