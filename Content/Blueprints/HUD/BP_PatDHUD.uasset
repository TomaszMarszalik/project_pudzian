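; BP_PatDHUD is a HUD Blueprint that shows the debug menu and hides it during combat.
; On BeginPlay it creates a WBP_Debug widget for the first player controller and adds it to the viewport.
; It then finds the BP_CombatSystem actor and binds to its combat start and end events to toggle the widget between hidden and visible.
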(event `self.ReceiveBeginPlay`
  (bind _returnvalue (`|CreateWidget` "/Game/Blueprints/HUD/Debug_Menu/WBP_Debug.WBP_Debug_C" (`GameplayStatics.GetPlayerController` 0)))
  (bind _output_get (set `self.debug nenu ref` _returnvalue))
  (`UserWidget.AddToViewport` _output_get 0)
  (bind _returnvalue_2 (`GameplayStatics.GetActorOfClass` "/Game/Blueprints/Core/Combat/BP_CombatSystem.BP_CombatSystem_C"))
  (add `/Game/Blueprints/Core/Combat/BP_CombatSystem.On Combat Start` _returnvalue_2 (delegate `Hide Debug Menu`))
  (add `/Game/Blueprints/Core/Combat/BP_CombatSystem.On Combat Ended` _returnvalue_2 (delegate `RestoreDebugMenu`)))

(event `RestoreDebugMenu`
  (`Widget.SetVisibility` (`self.debug nenu ref`) "Visible"))

(event `Hide Debug Menu`
  (`Widget.SetVisibility` (`self.debug nenu ref`) "Hidden"))

(fn `UserConstructionScript`)