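; Actor component that drives a top-down style camera through the owner's spring arm, handling pan, zoom and yaw rotation.
; Enhanced Input events adjust desired location along the arm's flattened right and forward vectors, a clamped desired arm length, and desired rotation.
; BeginPlay caches the spring arm and seeds these targets from its current state.
; Tick interpolates location and zoom toward them, while rotation is applied directly without smoothing.
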(event `EnhancedInput|/Game/TopDown/Input/Actions/IA_CameraHorizontal`
  (params (ActionValue :type "Float (double-precision)") (ElapsedSeconds :type "Float (double-precision)") (TriggeredSeconds :type "Float (double-precision)") (InputAction :type "InputAction Object Reference" :default "/Game/TopDown/Input/Actions/IA_CameraHorizontal.IA_CameraHorizontal"))
  (bind (_returnvalue_x _returnvalue_y) (`KismetMathLibrary.BreakVector` (`SceneComponent.GetRightVector` (`self.SpringArm`))))
  ;[1 1 1] Camera handling
  (:`Triggered`
    (set `self.Location_Desired` (+ (`self.Location_Desired`) (* (* ActionValue 20.0) (`KismetMathLibrary.MakeVector` _returnvalue_x _returnvalue_y))))))

(event `EnhancedInput|/Game/TopDown/Input/Actions/IA_CameraVertical`
  (params (ActionValue :type "Float (double-precision)") (ElapsedSeconds :type "Float (double-precision)") (TriggeredSeconds :type "Float (double-precision)") (InputAction :type "InputAction Object Reference" :default "/Game/TopDown/Input/Actions/IA_CameraVertical.IA_CameraVertical"))
  (bind (_returnvalue_x _returnvalue_y) (`KismetMathLibrary.BreakVector` (`SceneComponent.GetForwardVector` (`self.SpringArm`))))
  ;[1 1 1] Camera handling
  (:`Triggered`
    (set `self.Location_Desired` (+ (`self.Location_Desired`) (* (* ActionValue 20.0) (`KismetMathLibrary.MakeVector` _returnvalue_x _returnvalue_y))))))

(event `EnhancedInput|/Game/TopDown/Input/Actions/IA_CameraZoom`
  (params (ActionValue :type "Float (double-precision)") (ElapsedSeconds :type "Float (double-precision)") (TriggeredSeconds :type "Float (double-precision)") (InputAction :type "InputAction Object Reference" :default "/Game/TopDown/Input/Actions/IA_CameraZoom.IA_CameraZoom"))
  ;[1 1 1] Camera handling
  (:`Triggered`
    (set `self.Zoom_Desired` (`KismetMathLibrary.FClamp` (+ (* ActionValue 40.0) (`self.Zoom_Desired`)) 300.0 1500.0))))

(event `EnhancedInput|/Game/TopDown/Input/Actions/IA_CameraRotation`
  (params (ActionValue :type "Float (double-precision)") (ElapsedSeconds :type "Float (double-precision)") (TriggeredSeconds :type "Float (double-precision)") (InputAction :type "InputAction Object Reference" :default "/Game/TopDown/Input/Actions/IA_CameraRotation.IA_CameraRotation"))
  ;[1 1 1] Camera handling
  (:`Triggered`
    (set `self.Rotation_Desired` (`KismetMathLibrary.ComposeRotators` (`SceneComponent.K2_GetComponentRotation` (`self.SpringArm`)) (`KismetMathLibrary.MakeRotator` 0.0 0.0 (* ActionValue 5.0))))))

(event `self.ReceiveTick`
  (params (DeltaSeconds :type "Float (single-precision)"))
  (bind _springarm (`self.SpringArm`))
  (bind _springarm_2 (`self.SpringArm`))
  ;[1 1 1] Camera handling
  (set `SpringArmComponent.TargetArmLength` (`KismetMathLibrary.FInterpTo` (`SpringArmComponent.TargetArmLength` _springarm) (`self.Zoom_Desired`) DeltaSeconds 2.0) _springarm)
  (`SceneComponent.K2_SetWorldLocation` _springarm_2 (`KismetMathLibrary.VInterpTo` (`SceneComponent.K2_GetComponentLocation` _springarm_2) (`self.Location_Desired`) DeltaSeconds 5.0) false false)
  (`SceneComponent.K2_SetWorldRotation` (`self.SpringArm`) (`self.Rotation_Desired`) false false))

(event `self.ReceiveBeginPlay`
  (bind _springarm (`self.SpringArm`))
  (bind _returnvalue (`Actor.GetComponentByClass` (`self.GetOwner`) "/Script/Engine.SpringArmComponent"))
  ;[1 1 1] Camera handling initialization
  (`/Engine/EditorBlueprintResources/StandardMacros.IsValid` _returnvalue
    (:`Is Valid`
      (set `self.SpringArm` _returnvalue)
      (set `self.Location_Desired` (`SceneComponent.K2_GetComponentLocation` _springarm))
      (set `self.Zoom_Desired` (`SpringArmComponent.TargetArmLength` _springarm))
      (set `self.Rotation_Desired` (`SceneComponent.K2_GetComponentRotation` (`self.SpringArm`))))))