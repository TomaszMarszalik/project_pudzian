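; Combat manager for a tile-based tactics game, tracking units on BP_Grid, their teams and the turn-based fight from start to finish.
; It keeps tile occupancy synced with grid changes, cycles turns through living characters and charges movement path cost as tokens.
; Actions resolve pattern-based range and AoE, filtered by walkability and optional offset line-of-sight traces, then spawn an animation actor and apply hits.
; A death that leaves one team standing triggers combat finish.
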(event `self.ReceiveBeginPlay`
  (bind _grid_ref (`self.Grid Ref`))
  (add `/Game/Blueprints/Grid/BP_Grid.OnGridGenerated` _grid_ref (`|CreateDelegate` :!event `Update The Units on Grid Regen`))
  (add `/Game/Blueprints/Grid/BP_Grid.OnTileDataUpdated` _grid_ref (`|CreateDelegate` :!event `Update The Units on Tile Update`)))

(fn `Add Unit On Grid`
  (params (Character :type "/Game/Blueprints/Characters/BP_Character Object Reference") (Index :type "IntPoint Structure") (`Team Index` :type Integer))
  (`KismetArrayLibrary.Array_Add` (`self.Characters on Grid`) Character)
  (`self.Set Unit Index on Grid` Character Index)
  (`/Game/Blueprints/Characters/BP_Character.Set Grid` (`local.Character`) (`self.Grid Ref`))
  (add `/Game/Blueprints/Characters/BP_Character.On Character Reach New Tile` (`local.Character`) (`|CreateDelegate` :!event `Unit reached new Tile`))
  (`self.Set Character Team Index` (`local.Character`) (`local.Team Index`)))

(fn `Can Start Combat`
  (returns (`Can Start Combat` :type Boolean) (`Enough Units` :type Boolean) (`Enough Teams` :type Boolean) (`Not in Combat` :type Boolean))
  (bind _returnvalue (not (`self.Is In Combat`)))
  (bind _returnvalue_2 (>= (`BlueprintMapLibrary.Map_Length` (`self.Teams`)) 2))
  (bind _returnvalue_3 (>= (`KismetArrayLibrary.Array_Length` (`self.Characters on Grid`)) 2))
  (return (and _returnvalue_3 _returnvalue_2 _returnvalue) _returnvalue_3 _returnvalue_2 _returnvalue))

(fn `Change Current Character`
  (locals (`Current Index` :type Integer :default 0) (`Next Living Character` :type "/Game/Blueprints/Characters/BP_Character Object Reference"))
  (bind _current_character (`self.Current Character`))
  (bind _output (`|GetArrayItem` (`self.Characters on Grid`) (`local.Current Index`)))
  (`|ExecutionSequence`
    (:`then_0`
      (`/Engine/EditorBlueprintResources/StandardMacros.IsValid` _current_character
        (:`Is Valid`
          (`/Game/Blueprints/Characters/BP_Character.End Turn` _current_character)
          (`self.On Character Turn Ended` (`self.Current Character`)))))
    (:`then_1`
      (set `local.Current Index` (`KismetArrayLibrary.Array_Find` (`self.Characters on Grid`) (`self.Current Character`)))
      (while (not (`KismetSystemLibrary.IsValid` (`local.Next Living Character`)))
        (set `local.Current Index` (mod (+ (`local.Current Index`) 1) (`KismetArrayLibrary.Array_Length` (`self.Characters on Grid`))))
        (if (not (`/Game/Blueprints/Characters/BP_Character.Check is Dead` _output))
          (set `local.Next Living Character` _output)))
      (bind _output_get (set `self.Current Character` (`local.Next Living Character`)))
      (`/Game/Blueprints/Characters/BP_Character.Start Turn` _output_get)
      (`self.On Character Turn Started` _output_get))))

(fn `End Combat`
  (set `self.Is In Combat` false)
  (set `self.Is Finishing Combat` false)
  (set `self.Current Character` null)
  (for _array_element (`self.Characters on Grid`)
    (`/Game/Blueprints/Characters/BP_Character.End Combat For Character` _array_element))
  (`self.On Combat Ended`))

(fn `Finish Combat`
  (params (`Wining Team  Index` :type Integer))
  (set `self.Is Finishing Combat` true)
  (`self.On Finishing Combat` `Wining Team  Index`))

(fn `Get Action Range`
  (params (`Cast ` :type "/Game/Blueprints/Core/Combat/Actions/Utility/F_ActionDataCast Structure") (`Origin Index` :type "IntPoint Structure"))
  (returns (`Indexes in Range` :type "Array of IntPoint Structure"))
  (locals (`Range Indexes` :type "Array of IntPoint Structure"))
  (bind (_pattern _range _requriessight) (break `/Game/Blueprints/Core/Combat/Actions/Utility/F_ActionDataCast` `Cast `))
  (bind _range_indexes (`/Game/Blueprints/Core/Combat/Actions/Utility/BFL_Actions.Get Grid Indexes From Pattern` (`/Game/Blueprints/Grid/BP_Grid.Tile Shape` (`self.Grid Ref`)) _pattern (`local.Origin Index`) _range))
  (bind _indexes_with_line_of_sight (`self.Remove Not Valid Indexes` _range_indexes))
  (set `local.Range Indexes` _indexes_with_line_of_sight)
  (if _requriessight
    (bind _indexes_with_line_of_sight_2 (`self.Remove Indexes without line of Sight` (`local.Origin Index`) (`local.Range Indexes`) (`local.Cast `)))
    (return _indexes_with_line_of_sight_2)
    (else
      (return (`local.Range Indexes`)))))

(fn `Get Health Modifier`
  (params (`Damage Value` :type Integer))
  (returns (`Modifier Value` :type Integer))
  (return `Damage Value`))

(fn `Has Line of Sight?`
  (params (`Origin Index` :type "IntPoint Structure") (`Target  Index` :type "IntPoint Structure") (Cast :type "/Game/Blueprints/Core/Combat/Actions/Utility/F_ActionDataCast Structure"))
  (returns (`Return Value` :type Boolean))
  (locals (`Origin Tile` :type "/Game/Blueprints/Grid/F_TileData Structure") (`Target Tile` :type "/Game/Blueprints/Grid/F_TileData Structure") (Start :type "Vector Structure") (End :type "Vector Structure"))
  (bind _grid_tiles_data (`/Game/Blueprints/Grid/BP_Grid.Grid Tiles Data` (`self.Grid Ref`)))
  (bind _returnvalue (`KismetMathLibrary.MakeVector` 0.0 0.0 (`.UnitHeight_12_A599C0254B3DD9832DF652928F4A4DE8` (break `/Game/Blueprints/Core/Combat/Actions/Utility/F_ActionDataCast` (`local.Cast`)))))
  (bind (_returnvalue_x _returnvalue_y) (`KismetMathLibrary.BreakVector` (* (`/Game/Blueprints/Grid/BP_Grid.Tile Size` (`self.Grid Ref`)) (`.LineofSightOffset_14_7D049B0C4B1379C23975568B52066420` (break `/Game/Blueprints/Core/Combat/Actions/Utility/F_ActionDataCast` (`local.Cast`))))))
  (bind _output_get (set `local.Origin Tile` (`BlueprintMapLibrary.Map_Find` _grid_tiles_data (`local.Origin Index`))))
  (if (`/Game/Blueprints/Grid/BP_Grid.Is Index Valid` (`self.Grid Ref`) (`.Index_10_EBED7CD648D9AC57BB540D8281F68B1E` (break `/Game/Blueprints/Grid/F_TileData` _output_get)))
    (bind _output_get_2 (set `local.Target Tile` (`BlueprintMapLibrary.Map_Find` _grid_tiles_data (`local.Target  Index`))))
    (if (`/Game/Blueprints/Grid/BP_Grid.Is Index Valid` (`self.Grid Ref`) (`.Index_10_EBED7CD648D9AC57BB540D8281F68B1E` (break `/Game/Blueprints/Grid/F_TileData` _output_get_2)))
      (set `local.Start` (+ (.location (`.TileTransform_9_C8B49F424080CB25DC8191A7EE85CF00` (break `/Game/Blueprints/Grid/F_TileData` (`local.Origin Tile`)))) _returnvalue))
      (set `local.End` (+ _returnvalue (.location (`.TileTransform_9_C8B49F424080CB25DC8191A7EE85CF00` (break `/Game/Blueprints/Grid/F_TileData` (`local.Target Tile`))))))
      (for _array_element (`|MakeArray` (`KismetMathLibrary.MakeVector2D` _returnvalue_x) (`KismetMathLibrary.MakeVector2D` (- 0.0 _returnvalue_x)) (`KismetMathLibrary.MakeVector2D` 0.0 _returnvalue_y) (`KismetMathLibrary.MakeVector2D` 0.0 (- 0.0 _returnvalue_y)))
        (bind (_x _y) (`KismetMathLibrary.BreakVector2D` _array_element))
        (bind (_outhit _returnvalue_2) (`KismetSystemLibrary.LineTraceSingle` (+ (`KismetMathLibrary.MakeVector` _x _y) (`local.Start`)) (`local.End`) "TraceTypeQuery6" false (`|MakeArray` (`.UnitonTile_19_090F5A1342BB3758B627C38D844712AB` (break `/Game/Blueprints/Grid/F_TileData` (`local.Origin Tile`))) (`.UnitonTile_19_090F5A1342BB3758B627C38D844712AB` (break `/Game/Blueprints/Grid/F_TileData` (`local.Target Tile`))) :!type "Actor Object Reference")))
        (if (not _returnvalue_2)
          (return true)))
      (return false))))

(fn `Perform Action`
  (params (Action :type "/Game/Blueprints/Core/Combat/Actions/Utility/Enum_Actions Enum" :default "NewEnumerator0") (`Origin Index` :type "IntPoint Structure") (`Target Index` :type "IntPoint Structure"))
  (locals (Data :type "/Game/Blueprints/Core/Combat/Actions/Utility/F_ActionsData Structure") (`Attacked indexes` :type "Array of IntPoint Structure") (`Impact Data` :type "/Game/Blueprints/Core/Combat/Actions/Utility/F_ActionImpact Structure") (Character :type "/Game/Blueprints/Characters/BP_Character Object Reference") (Anim :type "/Game/Blueprints/Core/Combat/Actions/BP_ActionAnimation Object Reference"))
  (bind _character (`local.Character`))
  (bind _damagevalue (break `/Game/Blueprints/Core/Combat/Actions/Utility/F_ActionImpact` (`.ImpactData_16_2A6944184758C49277D58CA8095E19F1` (break `/Game/Blueprints/Core/Combat/Actions/Utility/F_ActionsData` (`local.Data`)))))
  (bind (_index _tiletype _tiletransform _tilestate _unitontile) (break `/Game/Blueprints/Grid/F_TileData` (`BlueprintMapLibrary.Map_Find` (`/Game/Blueprints/Grid/BP_Grid.Grid Tiles Data` (`self.Grid Ref`)) (`local.Origin Index`))))
  (bind (_index_2 _tiletype_2 _tiletransform_2 _tilestate_2 _unitontile_2) (break `/Game/Blueprints/Grid/F_TileData` (`BlueprintMapLibrary.Map_Find` (`/Game/Blueprints/Grid/BP_Grid.Grid Tiles Data` (`self.Grid Ref`)) (`local.Origin Index`))))
  (bind _action_data (`/Game/Blueprints/Core/Combat/Actions/Utility/BFL_Actions.Get Action Data from Action` Action))
  (set `local.Data` _action_data)
  (`/Engine/EditorBlueprintResources/StandardMacros.IsValid` _unitontile
    (:`Is Valid`
      (bind _can_cast (`/Game/Blueprints/Characters/BP_Character.Can do Action` _unitontile (`local.Data`)))
      (if _can_cast
        (bind _indexes_in_range (`self.Get Action Range` (`.Cast_9_34DC641C48EEF71540EB4F8612D7E5A9` (break `/Game/Blueprints/Core/Combat/Actions/Utility/F_ActionsData` (`local.Data`))) (`local.Origin Index`) :!label _label))
        (if (`KismetArrayLibrary.Array_Contains` _indexes_in_range (`local.Target Index`))
          (if (== (`.Pattern_4_054FE0B842C02253818A8BA1266E999B` (break `/Game/Blueprints/Core/Combat/Actions/Utility/F_ActionDataCast` (`.CastAoe_12_8BEAF7DB45C178191E4109AC33170E73` (break `/Game/Blueprints/Core/Combat/Actions/Utility/F_ActionsData` (`local.Data`))))) 0)
            (set `local.Attacked indexes` (`|MakeArray` (`local.Target Index`)))
            (else
              (bind _indexes_in_range_2 (`self.Get Action Range` (`.CastAoe_12_8BEAF7DB45C178191E4109AC33170E73` (break `/Game/Blueprints/Core/Combat/Actions/Utility/F_ActionsData` (`local.Data`))) (`local.Target Index`)))
              (set `local.Attacked indexes` _indexes_in_range_2)))
          (bind _returnvalue (`|SpawnActorFromClass` (`.Animation_11_CDEA5A7A4C6BE8B513ABACA4801D2972` (break `/Game/Blueprints/Core/Combat/Actions/Utility/F_ActionsAssets` (`.ActionAssets_6_E3ADE61040E66190C7189FA99A660D8E` (break `/Game/Blueprints/Core/Combat/Actions/Utility/F_ActionsData` (`local.Data`))))) (`KismetMathLibrary.MakeTransform` (0.0 0.0 0.0)) "Undefined" "MultiplyWithRoot" null (`self.Grid Ref`) (`local.Origin Index`) (`local.Attacked indexes`) (`local.Target Index`) (struct) null null))
          (set `local.Anim` _returnvalue)
          (`|ExecutionSequence`
            (:`then_0`
              (`/Engine/EditorBlueprintResources/StandardMacros.IsValid` _unitontile_2
                (:`Is Valid`
                  (`/Game/Blueprints/Characters/BP_Character.Do Action` _unitontile_2 (`local.Target Index`)))))
            (:`then_1`
              (set `local.Impact Data` (make `/Game/Blueprints/Core/Combat/Actions/Utility/F_ActionImpact` _damagevalue (`self.Get Health Modifier` _damagevalue)))
              (for _array_element (`local.Attacked indexes`)
                (bind _output_get (set `local.Character` (`.UnitonTile_19_090F5A1342BB3758B627C38D844712AB` (break `/Game/Blueprints/Grid/F_TileData` (`BlueprintMapLibrary.Map_Find` (`/Game/Blueprints/Grid/BP_Grid.Grid Tiles Data` (`self.Grid Ref`)) _array_element)))))
                (`/Engine/EditorBlueprintResources/StandardMacros.IsValid` _output_get
                  (:`Is Valid`
                    (`/Game/Blueprints/Characters/BP_Character.Character Hit By Action` (`local.Character`) (`local.Impact Data`) (`local.Anim`))
                    (if (`/Game/Blueprints/Characters/BP_Character.Check is Dead` _character)
                      (`self.Process Death` _character)
                      (if (`self.Is Finishing Combat`)
                        (return))))))
              (if (`/Game/Blueprints/Characters/BP_Character.Check is Dead` (`self.Current Character`))
                (`self.Change Current Character`)))))))
    (:`Is Not Valid`
      (goto _label))))

(fn `Process Death`
  (params (Character :type "/Game/Blueprints/Characters/BP_Character Object Reference"))
  (locals (`Team Index` :type Integer) (`Teams still in combat` :type "Array of Integer"))
  (bind _teams_still_in_combat (`local.Teams still in combat`))
  (`self.Set Unit Index on Grid` Character (make `IntPoint` -999 -999) false false)
  (bind _keys (`BlueprintMapLibrary.Map_Keys` (`self.Teams`)))
  (for _array_element _keys
    (bind _output_get (set `local.Team Index` _array_element))
    (bind _result (`BlueprintSetLibrary.Set_ToArray` (`.CharacterSet_3_902F49894C9D7ECA3B26B1A28DC02583` (break `/Game/Blueprints/Core/Combat/F_CharacterSet` (`BlueprintMapLibrary.Map_Find` (`self.Teams`) _output_get)))))
    (for _array_element_2 _result
      (if (not (`/Game/Blueprints/Characters/BP_Character.Check is Dead` _array_element_2))
        (`KismetArrayLibrary.Array_Add` (`local.Teams still in combat`) (`local.Team Index`))
        (break))))
  (if (not (!= (`KismetArrayLibrary.Array_Length` _teams_still_in_combat) 1))
    (`self.Finish Combat` (`|GetArrayItem` _teams_still_in_combat))))

(fn `Remove Indexes without line of Sight`
  (params (`Origin Index` :type "IntPoint Structure") (Indexes :type "Array of IntPoint Structure") (Cast :type "/Game/Blueprints/Core/Combat/Actions/Utility/F_ActionDataCast Structure"))
  (returns (`Indexes with Line of Sight` :type "Array of IntPoint Structure"))
  (locals (Ret :type "Array of IntPoint Structure"))
  (for _array_element Indexes
    (if (`self.Has Line of Sight?` (`local.Origin Index`) _array_element Cast)
      (`KismetArrayLibrary.Array_Add` (`local.Ret`) _array_element)))
  (return (`local.Ret`)))

(fn `Remove Not Valid Indexes`
  (params (Indexes :type "Array of IntPoint Structure"))
  (returns (`Indexes with Line of Sight` :type "Array of IntPoint Structure"))
  (locals (Ret :type "Array of IntPoint Structure"))
  (for _array_element Indexes
    (if (`/Game/Blueprints/Grid/BP_Grid.Is Tile Walkable` (`self.Grid Ref`) _array_element)
      (`KismetArrayLibrary.Array_Add` (`local.Ret`) _array_element)))
  (return (`local.Ret`)))

(fn `Remove Unit On Grid`
  (params (Character :type "/Game/Blueprints/Characters/BP_Character Object Reference") (`Destroy Unit` :type Boolean))
  (`self.Set Character Team Index` (`local.Character`) -1)
  (`KismetArrayLibrary.Array_RemoveItem` (`self.Characters on Grid`) Character)
  (`self.Set Unit Index on Grid` Character (make `IntPoint` -999 -999))
  (if `Destroy Unit`
    (`self.K2_DestroyActor` (`local.Character`))))

(fn `Set Character Team Index`
  (params (Character :type "/Game/Blueprints/Characters/BP_Character Object Reference") (`Team Index` :type Integer))
  (locals (`Character Set` :type "Set of /Game/Blueprints/Characters/BP_Character Object Reference"))
  (if (`.ReturnValue` (`BlueprintMapLibrary.Map_Find` (`/Game/Blueprints/Grid/BP_Grid.Grid Tiles Data` (`self.Grid Ref`)) (`/Game/Blueprints/Characters/BP_Character.Grid Index` (`local.Character`))))
    (`|ExecutionSequence`
      (:`then_0`
        (if (!= (`/Game/Blueprints/Characters/BP_Character.Team Index` (`local.Character`)) -1)
          (bind _output_get (set `local.Character Set` (`.CharacterSet_3_902F49894C9D7ECA3B26B1A28DC02583` (break `/Game/Blueprints/Core/Combat/F_CharacterSet` (`BlueprintMapLibrary.Map_Find` (`self.Teams`) (`/Game/Blueprints/Characters/BP_Character.Team Index` (`local.Character`)))))))
          (`BlueprintSetLibrary.Set_Remove` _output_get (`local.Character`))
          (if (> (`BlueprintSetLibrary.Set_Length` (`local.Character Set`)) 0)
            (`BlueprintMapLibrary.Map_Add` (`self.Teams`) (`/Game/Blueprints/Characters/BP_Character.Team Index` (`local.Character`)) (make `/Game/Blueprints/Core/Combat/F_CharacterSet` (`local.Character Set`)))
            (else
              (`BlueprintMapLibrary.Map_Remove` (`self.Teams`) (`/Game/Blueprints/Characters/BP_Character.Team Index` (`local.Character`)))))))
      (:`then_1`
        (if (!= (`local.Team Index`) -1)
          (bind _output_get_2 (set `local.Character Set` (`.CharacterSet_3_902F49894C9D7ECA3B26B1A28DC02583` (break `/Game/Blueprints/Core/Combat/F_CharacterSet` (`BlueprintMapLibrary.Map_Find` (`self.Teams`) (`local.Team Index`))))))
          (`BlueprintSetLibrary.Set_Add` _output_get_2 (`local.Character`))
          (`BlueprintMapLibrary.Map_Add` (`self.Teams`) (`local.Team Index`) (make `/Game/Blueprints/Core/Combat/F_CharacterSet` (`local.Character Set`)))))
      (:`then_2`
        (`/Game/Blueprints/Characters/BP_Character.Set Team Index` (`local.Character`) (`local.Team Index`) :!label _label)
        (`self.On Unit Team Change`)))
    (else
      (goto _label))))

(fn `Set Unit Index on Grid`
  (params (Character :type "/Game/Blueprints/Characters/BP_Character Object Reference") (Index :type "IntPoint Structure") (Force :type Boolean) (`Snap Actor` :type Boolean :default true))
  (locals (`Previous Tile` :type "/Game/Blueprints/Grid/F_TileData Structure"))
  (bind (_value _returnvalue) (`BlueprintMapLibrary.Map_Find` (`/Game/Blueprints/Grid/BP_Grid.Grid Tiles Data` (`self.Grid Ref`)) (`local.Index`)))
  (`|ExecutionSequence`
    (:`then_0`
      (if (or (!= (`/Game/Blueprints/Characters/BP_Character.Grid Index` (`local.Character`)) (`local.Index`)) (`local.Force`))
        (`|ExecutionSequence`
          (:`then_0`
            (bind _output_get (set `local.Previous Tile` (`BlueprintMapLibrary.Map_Find` (`/Game/Blueprints/Grid/BP_Grid.Grid Tiles Data` (`self.Grid Ref`)) (`/Game/Blueprints/Characters/BP_Character.Grid Index` (`local.Character`)))))
            (if (== (`local.Character`) (`.UnitonTile_19_090F5A1342BB3758B627C38D844712AB` (break `/Game/Blueprints/Grid/F_TileData` _output_get)))
              (bind _structout (setmembers `/Game/Blueprints/Grid/F_TileData` :`StructRef` (`local.Previous Tile`) :`Unit on Tile` null))
              (`BlueprintMapLibrary.Map_Add` (`/Game/Blueprints/Grid/BP_Grid.Grid Tiles Data` (`self.Grid Ref`)) (`.Index_10_EBED7CD648D9AC57BB540D8281F68B1E` (break `/Game/Blueprints/Grid/F_TileData` _structout)) _structout)))
          (:`then_1`
            (bind _output_get_2 (set `/Game/Blueprints/Characters/BP_Character.Grid Index` (`local.Index`) (`local.Character`)))
            (if (!= _output_get_2 (make `IntPoint` -999 -999))
              (bind _structout_2 (setmembers `/Game/Blueprints/Grid/F_TileData` :`StructRef` (`BlueprintMapLibrary.Map_Find` (`/Game/Blueprints/Grid/BP_Grid.Grid Tiles Data` (`self.Grid Ref`)) (`local.Index`)) :`Unit on Tile` (`local.Character`)))
              (`BlueprintMapLibrary.Map_Add` (`/Game/Blueprints/Grid/BP_Grid.Grid Tiles Data` (`self.Grid Ref`)) (`.Index_10_EBED7CD648D9AC57BB540D8281F68B1E` (break `/Game/Blueprints/Grid/F_TileData` _structout_2)) _structout_2)))
          (:`then_2`
            (`self.On Character Grid Index Change` (`local.Character`))))))
    (:`then_1`
      (if `Snap Actor`
        (`self.K2_SetActorLocation` (`local.Character`) (select `bool` _returnvalue :`false` (-999.0 -999.0 -999.0) :`true` (.location (`.TileTransform_9_C8B49F424080CB25DC8191A7EE85CF00` (break `/Game/Blueprints/Grid/F_TileData` _value)))) false false)))))

(fn `Start Combat`
  (set `self.Is In Combat` true)
  (for _array_element (`self.Characters on Grid`)
    (`/Game/Blueprints/Characters/BP_Character.Start Combat For Character` _array_element))
  (`self.On Combat Start`)
  (set `self.Current Character` null)
  (`self.Change Current Character`))

(fn `Unit reached new Tile`
  (params (Character :type "/Game/Blueprints/Characters/BP_Character Object Reference") (Index :type "IntPoint Structure")))

(fn `Update The Units on Grid Regen`
  (locals (NewLocalVar :type "Array of /Game/Blueprints/Characters/BP_Character Object Reference"))
  (bind _output_get (set `local.NewLocalVar` (`self.Characters on Grid`)))
  (for _array_element _output_get
    (bind _grid_index (`/Game/Blueprints/Characters/BP_Character.Grid Index` _array_element))
    (if (`/Game/Blueprints/Grid/BP_Grid.Is Tile Walkable` (`self.Grid Ref`) _grid_index)
      (`self.Set Unit Index on Grid` _array_element _grid_index true)
      (else
        (`self.Remove Unit On Grid` _array_element)))))

(fn `Update The Units on Tile Update`
  (params (Index :type "IntPoint Structure"))
  (locals (NewLocalVar :type "Array of /Game/Blueprints/Characters/BP_Character Object Reference"))
  (bind _output_get (set `local.NewLocalVar` (`self.Characters on Grid`)))
  (for _array_element _output_get
    (bind _grid_index (`/Game/Blueprints/Characters/BP_Character.Grid Index` _array_element))
    (if (`KismetMathLibrary.Equal_IntPointIntPoint` (`local.Index`) _grid_index)
      (if (`/Game/Blueprints/Grid/BP_Grid.Is Tile Walkable` (`self.Grid Ref`) _grid_index)
        (`self.Set Unit Index on Grid` _array_element _grid_index true)
        (break)
        (else
          (`self.Remove Unit On Grid` _array_element)
          (break))))))

(fn `UserConstructionScript`
  (bind _returnvalue (`GameplayStatics.GetActorOfClass` "/Game/Blueprints/Grid/BP_Grid.BP_Grid_C"))
  (set `self.Grid Ref` _returnvalue))

(fn `Validate Movement`
  (params (Character :type "/Game/Blueprints/Characters/BP_Character Object Reference") (Path :type "Array of IntPoint Structure"))
  (bind _path (`local.Path`))
  (if (> (`KismetArrayLibrary.Array_Length` Path) 0)
    (`/Game/Blueprints/Characters/BP_Character.Follow Path` (`local.Character`) Path)
    (bind _cost (`/Game/Blueprints/Characters/BP_Pathfinding.Get Path Cost` (`/Game/Blueprints/Grid/BP_Grid.As BP Pathfinding` (`self.Grid Ref`)) (`local.Path`)))
    (`/Game/Blueprints/Characters/BP_Character.Modify Current Tokens` (`local.Character`) (- 0 _cost) "NewEnumerator0")
    (`self.Set Unit Index on Grid` (`local.Character`) (`|GetArrayItem` _path (`KismetArrayLibrary.Array_LastIndex` _path)))))