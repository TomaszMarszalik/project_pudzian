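; Action animation actor for grid combat that plays a debug visual for an action, then signals completion and destroys itself.
; On BeginPlay it spawns a red BP_DebugAnimShape for each attacked tile index, using the grid's mesh and the origin and target tile transforms.
; Only the first shape's completion event is bound, and it triggers the completed dispatcher for the whole action.
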(event `self.ReceiveBeginPlay`
  (`self.Do The Action`))

(event `Do The Action`
  (bind (_meshsize _mesh _flatmesh _meshmaterial) (break `/Game/Blueprints/Grid/F_GridShapeData` (`/Game/Blueprints/Grid/BP_Grid.Out Row` (`self.Grid`))))
  (for (_array_element _array_index) (`self.Attacked Indexes`)
    (bind _returnvalue (`|SpawnActorFromClass` "/Game/Blueprints/Core/Combat/Actions/Components/BP_DebugAnimShape.BP_DebugAnimShape_C" (`KismetMathLibrary.MakeTransform` (0.0 0.0 0.0)) "AlwaysSpawn" "MultiplyWithRoot" null _mesh _meshmaterial (struct :`R` 0.401042 :`A` 1.0) (`.TileTransform_9_C8B49F424080CB25DC8191A7EE85CF00` (break `/Game/Blueprints/Grid/F_TileData` (`BlueprintMapLibrary.Map_Find` (`/Game/Blueprints/Grid/BP_Grid.Grid Tiles Data` (`self.Grid`)) (`self.Origin Index`)))) (`.TileTransform_9_C8B49F424080CB25DC8191A7EE85CF00` (break `/Game/Blueprints/Grid/F_TileData` (`BlueprintMapLibrary.Map_Find` (`/Game/Blueprints/Grid/BP_Grid.Grid Tiles Data` (`self.Grid`)) _array_element))) null))
    (if (== _array_index 0)
      (add `/Game/Blueprints/Core/Combat/Actions/Components/BP_DebugAnimShape.On Debug Anim Completed` _returnvalue (delegate `On Debug anim Completed`)))))

(event `On Debug anim Completed`
  (params (NewParam :type "/Game/Blueprints/Core/Combat/Actions/Components/BP_DebugAnimShape Object Reference"))
  (`self.Action Animation Finnished`))

(event `Action Animation Finnished`
  (`self.On Action Animation Completed` self)
  (`self.K2_DestroyActor`))

(fn `UserConstructionScript`)