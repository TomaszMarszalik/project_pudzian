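; BP_DebugAnimShape is a debug actor that shows a mesh animating from an origin transform to a target transform.
; On BeginPlay it applies the given mesh and material with a random color, then plays the Debug timeline.
; The timeline drives the transform lerp and adds a height offset track plus a fixed vertical lift.
; When finished, it fires OnDebugAnimCompleted and destroys itself after a short delay.
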(event `self.ReceiveBeginPlay`
  (bind _animated_shape (`self.Animated Shape`))
  (`StaticMeshComponent.SetStaticMesh` _animated_shape (`self.New Mesh`))
  (`PrimitiveComponent.SetMaterial` _animated_shape 0 (`self.Material`))
  (`MeshComponent.SetVectorParameterValueOnMaterials` _animated_shape "Color" (`KismetMathLibrary.MakeVector` (`KismetMathLibrary.RandomFloat`) (`KismetMathLibrary.RandomFloat`) (`KismetMathLibrary.RandomFloat`)))
  (bind (_direction _debug_anim_alpha _height_offset) (`Timeline|debug` :!via `PlayFromStart`)
    (:`Update`
      (bind (_returnvalue_location _returnvalue_rotation _returnvalue_scale) (`KismetMathLibrary.BreakTransform` (`KismetMathLibrary.TLerp` (`self.Origin Transform`) (`self.Target Transform`) _debug_anim_alpha)))
      (`self.K2_SetActorTransform` (`KismetMathLibrary.MakeTransform` (+ _returnvalue_location (`KismetMathLibrary.MakeVector` 0.0 0.0 _height_offset) (0.0 0.0 50.0)) _returnvalue_rotation _returnvalue_scale)))
    (:`Finished`
      (`self.On Debug Anim Completed` null)
      (`KismetSystemLibrary.Delay` 0.25)
      (`self.K2_DestroyActor`))))

(fn `UserConstructionScript`)