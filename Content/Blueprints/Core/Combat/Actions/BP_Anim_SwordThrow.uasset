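; Combat action animation actor that flies a thrown sword across the grid from an origin tile to a target tile.
; DotheAction places it at the origin tile, facing the target using a look-at rotation computed from the two tile indices.
; The SwordAnim timeline lerps its location between the two tile transforms, then calls ActionAnimationFinnished when the timeline ends.
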(event `self.Do The Action`
  (bind (_returnvalue_x _returnvalue_y) (`KismetMathLibrary.BreakVector2D` (`KismetMathLibrary.Conv_IntPointToVector2D` (`self.Target indexes`))))
  (bind (_returnvalue_x_2 _returnvalue_y_2) (`KismetMathLibrary.BreakVector2D` (`KismetMathLibrary.Conv_IntPointToVector2D` (`self.Origin Index`))))
  (bind _grid_tiles_data (`/Game/Blueprints/Grid/BP_Grid.Grid Tiles Data` (`self.Grid`)))
  (`self.K2_SetActorLocationAndRotation` (.location (`.TileTransform_9_C8B49F424080CB25DC8191A7EE85CF00` (break `/Game/Blueprints/Grid/F_TileData` (`BlueprintMapLibrary.Map_Find` (`/Game/Blueprints/Grid/BP_Grid.Grid Tiles Data` (`self.Grid`)) (`self.Origin Index`))))) (`KismetMathLibrary.FindLookAtRotation` (`KismetMathLibrary.MakeVector` _returnvalue_x_2 _returnvalue_y_2) (`KismetMathLibrary.MakeVector` _returnvalue_x _returnvalue_y)))
  (bind (_direction _location_alpha) (`Timeline|Sword Anim` :!via `PlayFromStart`)
    (:`Update`
      (`self.K2_SetActorLocation` (`KismetMathLibrary.VLerp` (.location (`.TileTransform_9_C8B49F424080CB25DC8191A7EE85CF00` (break `/Game/Blueprints/Grid/F_TileData` (`BlueprintMapLibrary.Map_Find` _grid_tiles_data (`self.Origin Index`))))) (.location (`.TileTransform_9_C8B49F424080CB25DC8191A7EE85CF00` (break `/Game/Blueprints/Grid/F_TileData` (`BlueprintMapLibrary.Map_Find` _grid_tiles_data (`self.Target indexes`))))) _location_alpha)))
    (:`Finished`
      (`self.Action Animation Finnished`))))

(fn `UserConstructionScript`
  (`parent.UserConstructionScript`))