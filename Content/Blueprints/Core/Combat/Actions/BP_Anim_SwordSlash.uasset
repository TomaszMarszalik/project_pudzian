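; Grid combat action animation actor that plays a sword slash for an action.
; DotheAction places the actor on the origin tile from the grid data and yaws or orients it toward the target tile using the two grid indices.
; The SwordAnim timeline sets the relative rotation and scale of AnimScaleAndRotation on each update, then signals ActionAnimationFinnished when it ends.
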(event `self.Do The Action`
  (bind _anim_scaleandrotation (`self.Anim_ScaleAndRotation`))
  (bind (_returnvalue_x _returnvalue_y) (`KismetMathLibrary.BreakVector2D` (`KismetMathLibrary.Conv_IntPointToVector2D` (`self.Target indexes`))))
  (bind (_returnvalue_x_2 _returnvalue_y_2) (`KismetMathLibrary.BreakVector2D` (`KismetMathLibrary.Conv_IntPointToVector2D` (`self.Origin Index`))))
  (`self.K2_SetActorLocationAndRotation` (.location (`.TileTransform_9_C8B49F424080CB25DC8191A7EE85CF00` (break `/Game/Blueprints/Grid/F_TileData` (`BlueprintMapLibrary.Map_Find` (`/Game/Blueprints/Grid/BP_Grid.Grid Tiles Data` (`self.Grid`)) (`self.Origin Index`))))) (`KismetMathLibrary.FindLookAtRotation` (`KismetMathLibrary.MakeVector` _returnvalue_x_2 _returnvalue_y_2) (`KismetMathLibrary.MakeVector` _returnvalue_x _returnvalue_y)))
  (`Timeline|Sword Anim` :!via `PlayFromStart`
    (:`Update`
      (`SceneComponent.K2_SetRelativeRotation` _anim_scaleandrotation (`KismetMathLibrary.MakeRotator` 0.0) false false)
      (`SceneComponent.SetRelativeScale3D` _anim_scaleandrotation (0.0 0.0 0.0)))
    (:`Finished`
      (`self.Action Animation Finnished`))))

(fn `UserConstructionScript`
  (`parent.UserConstructionScript`))