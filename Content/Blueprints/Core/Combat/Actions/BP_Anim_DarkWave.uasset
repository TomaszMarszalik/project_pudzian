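; BP_Anim_DarkWave is a combat action animation actor for the Dark Wave action on the grid.
; On DotheAction it moves itself to the target tile's location, looked up in the Grid's tile data by TargetIndexes.
; A Timeline then drives the relative scale of its Scene component and calls ActionAnimationFinnished when it completes.
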(event `self.Do The Action`
  (`self.K2_SetActorLocation` (.location (`.TileTransform_9_C8B49F424080CB25DC8191A7EE85CF00` (break `/Game/Blueprints/Grid/F_TileData` (`BlueprintMapLibrary.Map_Find` (`/Game/Blueprints/Grid/BP_Grid.Grid Tiles Data` (`self.Grid`)) (`self.Target indexes`))))))
  (bind (_direction _scale) (`Timeline|Timeline` :!via `PlayFromStart`)
    (:`Update`
      (`SceneComponent.SetRelativeScale3D` (`self.Scene`) _scale))
    (:`Finished`
      (`self.Action Animation Finnished`))))

(fn `UserConstructionScript`
  (`parent.UserConstructionScript`))