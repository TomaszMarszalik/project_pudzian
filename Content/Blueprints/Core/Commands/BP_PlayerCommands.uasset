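; Player input actor for the tactical grid that tracks hovered and selected tiles and characters.
; Each tick a cursor trace finds the character or tile underneath and updates hover states.
; Left and right clicks delegate to swappable command actors spawned from classes, which receive hover changes and re-execute while the button is held.
; Grid and combat system events resync the selection, which toggles tile and character states and broadcasts tile changes.
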(event `Change Selected Actions`
  (`self.Set Selected Actions` (`self.Left Action`) (`self.Right Action`)))

(event `self.ReceiveBeginPlay`
  (bind _grid (`self.Grid`))
  (bind _returnvalue (`GameplayStatics.GetActorOfClass` "/Game/Blueprints/Grid/BP_Grid.BP_Grid_C"))
  (set `self.Grid` _returnvalue)
  (bind _returnvalue_2 (`GameplayStatics.GetActorOfClass` "/Game/Blueprints/Core/Combat/BP_CombatSystem.BP_CombatSystem_C"))
  (bind _output_get (set `self.Combat System` _returnvalue_2))
  (add `/Game/Blueprints/Core/Combat/BP_CombatSystem.On Character Grid Index Change` _output_get (`|CreateDelegate` :!event `Character Grid Index Change`))
  (add `/Game/Blueprints/Grid/BP_Grid.OnGridGenerated` _grid (`|CreateDelegate` :!event `Update On Grid Generated`))
  (add `/Game/Blueprints/Grid/BP_Grid.OnTileDataUpdated` _grid (`|CreateDelegate` :!event `Update on Tile Updated`))
  (`self.EnableInput` (`GameplayStatics.GetPlayerController` 0))
  (`self.Set Selected Actions` "/Game/Blueprints/Core/Commands/Characters/Command_PerformAction.Command_PerformAction_C" "/Game/Blueprints/Core/Commands/Grid/Command_ShowActionRangeFromUnit.Command_ShowActionRangeFromUnit_C"))

(event `self.ReceiveTick`
  (params (DeltaSeconds :type "Float (single-precision)"))
  (`self.UpdateTileUnderCursor`))

(event `EnhancedInput|/Game/Inputs/IA_ActionExecute`
  (params (ActionValue :type Boolean) (ElapsedSeconds :type "Float (double-precision)") (TriggeredSeconds :type "Float (double-precision)") (InputAction :type "InputAction Object Reference" :default "/Game/Inputs/IA_ActionExecute.IA_ActionExecute"))
  (:`Triggered`
    (if ActionValue
      (`self.UpdateTileUnderCursor`)
      (set `self.Left Click Down` true)
      (`/Engine/EditorBlueprintResources/StandardMacros.IsValid` (`self.Selected Left Click`)
        (:`Is Valid`
          (`/Game/Blueprints/Core/Commands/BP_Command.Execute Action` (`self.Selected Left Click`) (`self.Hovered Tile`) :!label _label)))
      (else
        (set `self.Left Click Down` false)))))

(event `On Hovered Tile`
  (bind _selected_right_click (`self.Selected Right Click`))
  (bind _selected_left_click (`self.Selected Left Click`))
  (`|ExecutionSequence`
    (:`then_0`
      (`/Engine/EditorBlueprintResources/StandardMacros.IsValid` _selected_left_click
        (:`Is Valid`
          (`/Game/Blueprints/Core/Commands/BP_Command.Execute Hovered Action` _selected_left_click (`self.Hovered Tile`))
          (if (`self.Left Click Down`)
            (goto _label)))))
    (:`then_1`
      (`/Engine/EditorBlueprintResources/StandardMacros.IsValid` _selected_right_click
        (:`Is Valid`
          (`/Game/Blueprints/Core/Commands/BP_Command.Execute Hovered Action` _selected_right_click (`self.Hovered Tile`))
          (if (`self.Right Click Down`)
            (`/Game/Blueprints/Core/Commands/BP_Command.Execute Action` (`self.Selected Right Click`) (`self.Hovered Tile`) :!label _label_2)))))))

(event `EnhancedInput|/Game/Inputs/IA_Action2Execute`
  (params (ActionValue :type Boolean) (ElapsedSeconds :type "Float (double-precision)") (TriggeredSeconds :type "Float (double-precision)") (InputAction :type "InputAction Object Reference" :default "/Game/Inputs/IA_Action2Execute.IA_Action2Execute"))
  (:`Triggered`
    (if ActionValue
      (`self.UpdateTileUnderCursor`)
      (set `self.Right Click Down` true)
      (`/Engine/EditorBlueprintResources/StandardMacros.IsValid` (`self.Selected Right Click`)
        (:`Is Valid`
          (goto _label_2)))
      (else
        (set `self.Right Click Down` false)))))

(fn `Character Grid Index Change`
  (params (Character :type "/Game/Blueprints/Characters/BP_Character Object Reference"))
  (if (== Character (`self.Selected Character`))
    (`self.Set Selected Tile and Character` (`/Game/Blueprints/Characters/BP_Character.Grid Index` (`local.Character`)))))

(fn `Get Character Under Cursor`
  (params (PlayerIndex :type Integer))
  (returns (Character :type "/Game/Blueprints/Characters/BP_Character Object Reference"))
  (bind (_hitresult _returnvalue) (`PlayerController.GetHitResultUnderCursorByChannel` (`GameplayStatics.GetPlayerController` PlayerIndex) "TraceTypeQuery5" false))
  (if _returnvalue
    (return (cast `/Game/Blueprints/Characters/BP_Character` (`.HitActor` (`GameplayStatics.BreakHitResult` _hitresult)) :!pure true))
    (else
      (bind _index (`/Game/Blueprints/Grid/BP_Grid.Get Tile Under Cursor` (`self.Grid`) (`local.PlayerIndex`)))
      (return (`.UnitonTile_19_090F5A1342BB3758B627C38D844712AB` (break `/Game/Blueprints/Grid/F_TileData` (`BlueprintMapLibrary.Map_Find` (`/Game/Blueprints/Grid/BP_Grid.Grid Tiles Data` (`self.Grid`)) _index)))))))

(fn `Set Selected Actions`
  (params (`Left Action` :type "/Game/Blueprints/Core/Commands/BP_Command Class Reference") (`Right Action` :type "/Game/Blueprints/Core/Commands/BP_Command Class Reference"))
  (bind _selected_left_click (`self.Selected Left Click`))
  (bind _left_action (`local.Left Action`))
  (bind _selected_right_click (`self.Selected Right Click`))
  (bind _right_action (`local.Right Action`))
  (`|ExecutionSequence`
    (:`then_0`
      (`/Engine/EditorBlueprintResources/StandardMacros.IsValid` _selected_left_click
        (:`Is Valid`
          (`self.K2_DestroyActor` _selected_left_click)
          (set `self.Selected Left Click` null))
        (:`Is Not Valid`
          _))
      (if (`KismetSystemLibrary.IsValidClass` _left_action)
        (bind _returnvalue (`|SpawnActorFromClass` _left_action (`KismetMathLibrary.MakeTransform` (0.0 0.0 0.0)) "AlwaysSpawn" "MultiplyWithRoot" null self null))
        (set `self.Selected Left Click` _returnvalue)))
    (:`then_1`
      (`/Engine/EditorBlueprintResources/StandardMacros.IsValid` _selected_right_click
        (:`Is Valid`
          (`self.K2_DestroyActor` _selected_right_click)
          (set `self.Selected Right Click` null))
        (:`Is Not Valid`
          _))
      (if (`KismetSystemLibrary.IsValidClass` _right_action)
        (bind _returnvalue_2 (`|SpawnActorFromClass` _right_action (`KismetMathLibrary.MakeTransform` (0.0 0.0 0.0)) "AlwaysSpawn" "MultiplyWithRoot" null self null))
        (set `self.Selected Right Click` _returnvalue_2)))))

(fn `Set Selected Tile and Character`
  (params (Index :type "IntPoint Structure") (Force :type Boolean))
  (locals (`New Character` :type "/Game/Blueprints/Characters/BP_Character Object Reference"))
  (bind _selected_character (`self.Selected Character`))
  (`|ExecutionSequence`
    (:`then_0`
      (if (or (!= (`local.Index`) (`self.Selected Tile`)) (`local.Force`))
        (`/Game/Blueprints/Grid/BP_Grid.removestatetotile` (`self.Grid`) (`self.Selected Tile`) "NewEnumerator2")
        (set `self.Selected Tile` (`local.Index`))
        (`/Game/Blueprints/Grid/BP_Grid.addstatetotile` (`self.Grid`) (`self.Selected Tile`) "NewEnumerator2")
        (else
          (`/Game/Blueprints/Grid/BP_Grid.removestatetotile` (`self.Grid`) (`self.Selected Tile`) "NewEnumerator2")
          (set `self.Selected Tile` (make `IntPoint` -999 -999))))
      (`self.On Selected Tile Change` (`self.Selected Tile`)))
    (:`then_1`
      (bind _output_get (set `local.New Character` (`.UnitonTile_19_090F5A1342BB3758B627C38D844712AB` (break `/Game/Blueprints/Grid/F_TileData` (`BlueprintMapLibrary.Map_Find` (`/Game/Blueprints/Grid/BP_Grid.Grid Tiles Data` (`self.Grid`)) (`self.Selected Tile`))))))
      (if (or (!= _output_get (`self.Selected Character`)) (`local.Force`))
        (`|ExecutionSequence`
          (:`then_0`
            (`/Engine/EditorBlueprintResources/StandardMacros.IsValid` _selected_character
              (:`Is Valid`
                (`/Game/Blueprints/Characters/BP_Character.Set is Selected` _selected_character false))))
          (:`then_1`
            (bind _output_get_2 (set `self.Selected Character` (`local.New Character`)))
            (`/Engine/EditorBlueprintResources/StandardMacros.IsValid` _output_get_2
              (:`Is Valid`
                (`/Game/Blueprints/Characters/BP_Character.Set is Selected` _output_get_2 true)))))))))

(fn `Update On Grid Generated`
  (if (`/Game/Blueprints/Grid/BP_Grid.Is Index Valid` (`self.Grid`) (`self.Hovered Tile`))
    (`self.Set Selected Tile and Character` (`self.Hovered Tile`) true)
    (else
      (`self.Set Selected Tile and Character` (make `IntPoint` -999 -999)))))

(fn `Update on Tile Updated`
  (params (Index :type "IntPoint Structure"))
  (if (`KismetMathLibrary.Equal_IntPointIntPoint` Index (`self.Hovered Tile`))
    (`self.Update On Grid Generated`)))

(fn `UpdateTileUnderCursor`
  (locals (`New Index` :type "IntPoint Structure"))
  (bind _hovered_character (`self.Hovered Character`))
  (`|ExecutionSequence`
    (:`then_0`
      (bind _character (`self.Get Character Under Cursor` 0))
      (if (!= _character (`self.Hovered Character`))
        (`/Engine/EditorBlueprintResources/StandardMacros.IsValid` _hovered_character
          (:`Is Valid`
            (`/Game/Blueprints/Characters/BP_Character.Set Is Hovered` _hovered_character false))
          (:`Is Not Valid`
            _))
        (bind _output_get (set `self.Hovered Character` null))
        (`/Engine/EditorBlueprintResources/StandardMacros.IsValid` _output_get
          (:`Is Valid`
            (`/Game/Blueprints/Characters/BP_Character.Set Is Hovered` _output_get true)))))
    (:`then_1`
      (`/Engine/EditorBlueprintResources/StandardMacros.IsValid` (`self.Hovered Character`)
        (:`Is Valid`
          (set `local.New Index` (`/Game/Blueprints/Characters/BP_Character.Grid Index` (`self.Hovered Character`))))
        (:`Is Not Valid`
          (bind _index (`/Game/Blueprints/Grid/BP_Grid.Get Tile Under Cursor` (`self.Grid`) 0))
          (set `local.New Index` _index)))
      (if (!= (`local.New Index`) (`self.Hovered Tile`))
        (`/Game/Blueprints/Grid/BP_Grid.removestatetotile` (`self.Grid`) (`self.Hovered Tile`) "NewEnumerator1")
        (set `self.Hovered Tile` (`local.New Index`))
        (`/Game/Blueprints/Grid/BP_Grid.addstatetotile` (`self.Grid`) (`self.Hovered Tile`) "NewEnumerator1")
        (`self.On Hovered Tile`)))))

(fn `UserConstructionScript`)