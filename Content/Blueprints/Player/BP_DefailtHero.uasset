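; Player hero Blueprint that provides a pannable, zoomable, rotatable spring-arm camera and a dice-based combat stance picker.
; Enhanced Input sets desired camera values, and Tick interpolates location and clamped zoom while applying rotation directly.
; Debug key C zeroes six dice and swaps the HUD for the stance widget.
; Stances 1 and 3 add Shadow or Iron form components, trigger their dice rolls and restore the HUD; stance 2 only closes the picker.
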(event Custom|Stance%203%20Choice_Event
  ;[0.4179 0.3278 0] Stance 3
  (Widget|RemovefromParent (Variables|Default|GetStance%20Choice))
  (bind _returnvalue (AddComponent|AddBPIronForm))
  (Default|ConstructionDiceRollIron _returnvalue)
  (bind _returnvalue_2 (UserInterface|CreateWidget "/Game/Blueprints/HUD/WBP_HeroHUD.WBP_HeroHUD_C" (Game|GetPlayerController 0)))
  (bind _output_get (Variables|Default|SetHero%20HUD _returnvalue_2))
  (UserInterface|Viewport|AddtoViewport _output_get 0))

(event Custom|Stance%201%20Choice_Event
  ;[0.4179 0.3278 0] Stance 1
  (Widget|RemovefromParent (Variables|Default|GetStance%20Choice))
  (bind _returnvalue (AddComponent|AddBPShadowForm))
  (Default|ConstructionDiceRollShadow _returnvalue)
  (bind _returnvalue_2 (UserInterface|CreateWidget "/Game/Blueprints/HUD/WBP_HeroHUD.WBP_HeroHUD_C" (Game|GetPlayerController 0)))
  (bind _output_get (Variables|Default|SetHero%20HUD _returnvalue_2))
  (UserInterface|Viewport|AddtoViewport _output_get 0))

(event Custom|Stance%202%20Choice_Event
  (Widget|RemovefromParent (Variables|Default|GetStance%20Choice)))

(event Input|EnhancedActionEvents|EnhancedInputActionIA_CameraZoom
  (params (ActionValue :type Float%20%28double-precision%29) (ElapsedSeconds :type Float%20%28double-precision%29) (TriggeredSeconds :type Float%20%28double-precision%29) (InputAction :type Input%20Action%20Object%20Reference :default "/Game/TopDown/Input/Actions/IA_CameraZoom.IA_CameraZoom"))
  ;[1 1 1] Camera handling
  (Variables|Default|SetZoom_Desired (Math|Float|Clamp(Float) (+ (* ActionValue 4e+01) (Variables|Default|GetZoom_Desired)) 3e+02 1.5e+03)))

(event Input|EnhancedActionEvents|EnhancedInputActionIA_CameraHorizontal
  (params (ActionValue :type Float%20%28double-precision%29) (ElapsedSeconds :type Float%20%28double-precision%29) (TriggeredSeconds :type Float%20%28double-precision%29) (InputAction :type Input%20Action%20Object%20Reference :default "/Game/TopDown/Input/Actions/IA_CameraHorizontal.IA_CameraHorizontal"))
  (bind _springarm (Variables|Camera|GetSpringArm))
  (bind _returnvalue (Math|Vector|GetRightVector _springarm))
  ;[1 1 1] Camera handling
  (Variables|Default|SetLocation_Desired (+ (Variables|Default|GetLocation_Desired) (* (* ActionValue 2e+01) (Math|Vector|MakeVector (.x _returnvalue) (.y _returnvalue) 0.0)))))

(event Input|EnhancedActionEvents|EnhancedInputActionIA_CameraVertical
  (params (ActionValue :type Float%20%28double-precision%29) (ElapsedSeconds :type Float%20%28double-precision%29) (TriggeredSeconds :type Float%20%28double-precision%29) (InputAction :type Input%20Action%20Object%20Reference :default "/Game/TopDown/Input/Actions/IA_CameraVertical.IA_CameraVertical"))
  (bind _springarm (Variables|Camera|GetSpringArm))
  (bind _returnvalue (Math|Vector|GetForwardVector _springarm))
  ;[1 1 1] Camera handling
  (Variables|Default|SetLocation_Desired (+ (Variables|Default|GetLocation_Desired) (* (* ActionValue 2e+01) (Math|Vector|MakeVector (.x _returnvalue) (.y _returnvalue) 0.0)))))

(event Input|EnhancedActionEvents|EnhancedInputActionIA_CameraRotation
  (params (ActionValue :type Float%20%28double-precision%29) (ElapsedSeconds :type Float%20%28double-precision%29) (TriggeredSeconds :type Float%20%28double-precision%29) (InputAction :type Input%20Action%20Object%20Reference :default "/Game/TopDown/Input/Actions/IA_CameraRotation.IA_CameraRotation"))
  ;[1 1 1] Camera handling
  (Variables|Default|SetRotation_Desired (Math|Rotator|CombineRotators (Transformation|GetWorldRotation (Variables|Camera|GetSpringArm)) (Math|Rotator|MakeRotator 0.0 0.0 (* ActionValue 5.0)))))

(event EventTick
  (params (DeltaSeconds :type Float%20%28single-precision%29))
  (bind _springarm (Variables|Camera|GetSpringArm))
  (bind _springarm_2 (Variables|Camera|GetSpringArm))
  ;[1 1 1] Camera handling
  (Variables|/Script/Engine.SpringArmComponent|SetTargetArmLength _springarm (Math|Interpolation|FInterpTo (Variables|/Script/Engine.SpringArmComponent|GetTargetArmLength _springarm) (Variables|Default|GetZoom_Desired) DeltaSeconds 2.0))
  (Transformation|SetWorldLocation _springarm_2 (Math|Interpolation|VInterpTo (Transformation|GetWorldLocation _springarm_2) (Variables|Default|GetLocation_Desired) DeltaSeconds 5.0) false false)
  (Transformation|SetWorldRotation (Variables|Camera|GetSpringArm) (Variables|Default|GetRotation_Desired) false false))

(event EventBeginPlay
  (bind _springarm (Variables|Camera|GetSpringArm))
  ;[0.2141 0 0.3333 1 24] Initilize HUD
  (bind _returnvalue (UserInterface|CreateWidget "/Game/Blueprints/HUD/WBP_HeroHUD.WBP_HeroHUD_C" (Game|GetPlayerController 0)))
  (bind _output_get (Variables|Default|SetHero%20HUD _returnvalue))
  (UserInterface|Viewport|AddtoViewport _output_get 0)
  ;[1 1 1] Camera handling initialization
  (Variables|Default|SetLocation_Desired (Transformation|GetWorldLocation _springarm))
  (Variables|Default|SetZoom_Desired (Variables|/Script/Engine.SpringArmComponent|GetTargetArmLength _springarm))
  (Variables|Default|SetRotation_Desired (Transformation|GetWorldRotation (Variables|Camera|GetSpringArm))))

(event Input|KeyboardEvents|DebugKeyC
  (params (Key :type Key%20Structure :default "None") (ActionValue :type Input%20Action%20Value%20Structure))
  ;[0.121 0.0189 0.349 1 24] Enable Stance Picker
  (:Pressed
    (Variables|Default|SetDie%201 0)
    (Variables|Default|SetDie%202 0)
    (Variables|Default|SetDie%203 0)
    (Variables|Default|SetDie%204 0)
    (Variables|Default|SetDie%205 0)
    (Variables|Default|SetDie%206 0)
    (Widget|RemovefromParent (Variables|Default|GetHero%20HUD))
    (bind _returnvalue (UserInterface|CreateWidget "/Game/Blueprints/HUD/WBP_StanceChoice.WBP_StanceChoice_C" (Game|GetPlayerController 0)))
    (bind _output_get (Variables|Default|SetStance%20Choice _returnvalue))
    (UserInterface|Viewport|AddtoViewport _output_get 0)))

(fn ConstructionScript)