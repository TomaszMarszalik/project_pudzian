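; BP_Range is a player targeting helper that finds targetable pawns overlapping its Range component.
; GetTargetInRange queries each overlapping pawn with an IsTargetable interface message, then separates out those absent from BP_TopDownController's RecentlyTargeted list.
; It returns those fresh targets, or clears that history and returns all targets when none are fresh, which supports cycling through targets.
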(fn `Get Target in range`
  (returns (`Possible Targets` :type "Array of Actor Object Reference"))
  (locals (Targets :type "Array of Actor Object Reference") (FreshTargets :type "Array of Actor Object Reference"))
  (bind _asbp_top_down_controller (cast `/Game/Blueprints/Core/BP_TopDownController` (`GameplayStatics.GetPlayerController` 0)))
  (set `self.As BP Top Down Controller` _asbp_top_down_controller)
  (for _array_element (`PrimitiveComponent.GetOverlappingActors` (`self.Range`) "/Script/Engine.Pawn")
    (bind _is_targetable (message `/Game/Blueprints/Player/I_TargetCheck.Is Targetable` _array_element))
    (if _is_targetable
      (`KismetArrayLibrary.Array_AddUnique` (`local.Targets`) _array_element)
      (if (not (`KismetArrayLibrary.Array_Contains` (`/Game/Blueprints/Core/BP_TopDownController.recently targeted` (`self.As BP Top Down Controller`)) _array_element))
        (`KismetArrayLibrary.Array_AddUnique` (`local.FreshTargets`) _array_element))))
  (if (`KismetArrayLibrary.Array_IsEmpty` (`local.FreshTargets`))
    (`KismetArrayLibrary.Array_Clear` (`/Game/Blueprints/Core/BP_TopDownController.recently targeted` (`self.As BP Top Down Controller`)))
    (return (`local.Targets`))
    (else
      (return (`local.FreshTargets`)))))

(fn `UserConstructionScript`)