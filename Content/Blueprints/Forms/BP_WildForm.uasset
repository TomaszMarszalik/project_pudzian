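; BP_WildForm is a form Blueprint that supplies the construction dice roll for the Wild form.
; Its one function fills the first three slots of the WildDice array with a random one-to-ten roll followed by two one-to-six rolls, then returns that array.
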(fn `ConstructionDiceRoll_Wild`
  (returns (`Power  Dice values` :type "Array of Integer"))
  (`KismetArrayLibrary.Array_Set` (`self.Wild Dice`) 0 (`KismetMathLibrary.RandomIntegerInRange` 1 10))
  (`KismetArrayLibrary.Array_Set` (`self.Wild Dice`) 1 (`KismetMathLibrary.RandomIntegerInRange` 1 6))
  (`KismetArrayLibrary.Array_Set` (`self.Wild Dice`) 2 (`KismetMathLibrary.RandomIntegerInRange` 1 6))
  (return (`self.Wild Dice`)))