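; BP_SongForm is a song form Blueprint that rolls a set of random dice for a song.
; Its ConstructionDiceRollSong function fills the first four slots of the SongDice array with independent rolls of one d8, two d6 and one d4, then returns the array.
; The file does not show how the results are used.
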(fn `ConstructionDiceRoll_Song`
  (returns (`Song Dice values` :type "Array of Integer"))
  (`KismetArrayLibrary.Array_Set` (`self.Song  Dice`) 0 (`KismetMathLibrary.RandomIntegerInRange` 1 8))
  (`KismetArrayLibrary.Array_Set` (`self.Song  Dice`) 1 (`KismetMathLibrary.RandomIntegerInRange` 1 6))
  (`KismetArrayLibrary.Array_Set` (`self.Song  Dice`) 2 (`KismetMathLibrary.RandomIntegerInRange` 1 6))
  (`KismetArrayLibrary.Array_Set` (`self.Song  Dice`) 3 (`KismetMathLibrary.RandomIntegerInRange` 1 4))
  (return (`self.Song  Dice`)))