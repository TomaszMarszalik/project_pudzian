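; BP_BlasterForm is a Blueprint for the Blaster form, containing a construction dice roll function.
; The function rolls three independent eight-sided dice as random integers and writes them into the first three slots of the BlasterDice array.
; It then returns that array to the caller.
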(fn `ConstructionDiceRoll_Blaster`
  (returns (`Shadow Dice values` :type "Array of Integer"))
  (`KismetArrayLibrary.Array_Set` (`self.Blaster Dice`) 0 (`KismetMathLibrary.RandomIntegerInRange` 1 8))
  (`KismetArrayLibrary.Array_Set` (`self.Blaster Dice`) 1 (`KismetMathLibrary.RandomIntegerInRange` 1 8))
  (`KismetArrayLibrary.Array_Set` (`self.Blaster Dice`) 2 (`KismetMathLibrary.RandomIntegerInRange` 1 8))
  (return (`self.Blaster Dice`)))