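; BP_PowerForm is a form Blueprint that supplies the construction dice roll for Power.
; ConstructionDiceRollPower overwrites the first three slots of the PowerDice array with random rolls, two ten-sided and one four-sided, then returns the array.
; The dice stay as separate values, with no summing or other use of the results in this graph.
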(fn `ConstructionDiceRoll_Power`
  (returns (`Power  Dice values` :type "Array of Integer"))
  (`KismetArrayLibrary.Array_Set` (`self.Power Dice`) 0 (`KismetMathLibrary.RandomIntegerInRange` 1 10))
  (`KismetArrayLibrary.Array_Set` (`self.Power Dice`) 1 (`KismetMathLibrary.RandomIntegerInRange` 1 10))
  (`KismetArrayLibrary.Array_Set` (`self.Power Dice`) 2 (`KismetMathLibrary.RandomIntegerInRange` 1 4))
  (return (`self.Power Dice`)))