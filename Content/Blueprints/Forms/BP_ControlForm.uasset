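; BP_ControlForm is a form Blueprint that provides a dice roll for Control, named as a construction roll.
; Its single function fills the first four slots of the ControlDice array with random integers from dice of descending size, d10 down to d4, then returns the array.
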(fn `ConstructionDiceRoll_Control`
  (returns (`Shadow Dice values` :type "Array of Integer"))
  (`KismetArrayLibrary.Array_Set` (`self.Control Dice`) 0 (`KismetMathLibrary.RandomIntegerInRange` 1 10))
  (`KismetArrayLibrary.Array_Set` (`self.Control Dice`) 1 (`KismetMathLibrary.RandomIntegerInRange` 1 8))
  (`KismetArrayLibrary.Array_Set` (`self.Control Dice`) 2 (`KismetMathLibrary.RandomIntegerInRange` 1 6))
  (`KismetArrayLibrary.Array_Set` (`self.Control Dice`) 3 (`KismetMathLibrary.RandomIntegerInRange` 1 4))
  (return (`self.Control Dice`)))