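; BP_DanceForm is a Dance form Blueprint that rolls a set of random dice values for dancing.
; Its ConstructionDiceRoll_Dance function writes a d10, a d8 and a d6 result into the first three slots of the DanceDice array, then returns that array.
; Each die is an independent random integer roll starting at one.
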(fn `ConstructionDiceRoll_Dance`
  (returns (`Shadow Dice values` :type "Array of Integer"))
  (`KismetArrayLibrary.Array_Set` (`self.Dance Dice`) 0 (`KismetMathLibrary.RandomIntegerInRange` 1 10))
  (`KismetArrayLibrary.Array_Set` (`self.Dance Dice`) 1 (`KismetMathLibrary.RandomIntegerInRange` 1 8))
  (`KismetArrayLibrary.Array_Set` (`self.Dance Dice`) 2 (`KismetMathLibrary.RandomIntegerInRange` 1 6))
  (return (`self.Dance Dice`)))