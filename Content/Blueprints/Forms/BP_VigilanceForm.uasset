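; BP_VigilanceForm is a form Blueprint whose single function rolls six-sided dice for Vigilance.
; ConstructionDiceRollVigilance writes random integers from 1 to 6 into the VigilanceDice array and returns it.
; It makes four rolls but writes index 2 twice, so only the first three slots are set and the third roll is overwritten.
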(fn `ConstructionDiceRoll_Vigilance`
  (returns (`Power  Dice values` :type "Array of Integer"))
  (`KismetArrayLibrary.Array_Set` (`self.Vigilance Dice`) 0 (`KismetMathLibrary.RandomIntegerInRange` 1 6))
  (`KismetArrayLibrary.Array_Set` (`self.Vigilance Dice`) 1 (`KismetMathLibrary.RandomIntegerInRange` 1 6))
  (`KismetArrayLibrary.Array_Set` (`self.Vigilance Dice`) 2 (`KismetMathLibrary.RandomIntegerInRange` 1 6))
  (`KismetArrayLibrary.Array_Set` (`self.Vigilance Dice`) 2 (`KismetMathLibrary.RandomIntegerInRange` 1 6))
  (return (`self.Vigilance Dice`)))