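; BP_OneTwoForm is a Blueprint that rolls a set of construction dice for the OneTwo form.
; ConstructionDiceRollOneTwo writes random 1–6 rolls into the first two slots of the OneTwoDice array and a 1–4 roll into the third, then returns the array.
; The third slot is set twice, so the second roll overwrites the first and no fourth slot is written.
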(fn `ConstructionDiceRoll_OneTwo`
  (returns (`Power  Dice values` :type "Array of Integer"))
  (`KismetArrayLibrary.Array_Set` (`self.OneTwo Dice`) 0 (`KismetMathLibrary.RandomIntegerInRange` 1 6))
  (`KismetArrayLibrary.Array_Set` (`self.OneTwo Dice`) 1 (`KismetMathLibrary.RandomIntegerInRange` 1 6))
  (`KismetArrayLibrary.Array_Set` (`self.OneTwo Dice`) 2 (`KismetMathLibrary.RandomIntegerInRange` 1 4))
  (`KismetArrayLibrary.Array_Set` (`self.OneTwo Dice`) 2 (`KismetMathLibrary.RandomIntegerInRange` 1 4))
  (return (`self.OneTwo Dice`)))