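; BP_ShadowForm is a form Blueprint that rolls the construction dice for the Shadow form.
; ConstructionDiceRollShadow writes random integers into the first four slots of the ShadowDice array, then returns the array.
; Each slot first gets a four-sided roll.
; The last two slots are then rolled again, with the third ending on a much wider 1 to 64 range that overwrites its earlier value.
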(fn `ConstructionDiceRoll_Shadow`
  (returns (`Shadow Dice values` :type "Array of Integer"))
  (`KismetArrayLibrary.Array_Set` (`self.Shadow Dice`) 0 (`KismetMathLibrary.RandomIntegerInRange` 1 4))
  (`KismetArrayLibrary.Array_Set` (`self.Shadow Dice`) 1 (`KismetMathLibrary.RandomIntegerInRange` 1 4))
  (`KismetArrayLibrary.Array_Set` (`self.Shadow Dice`) 2 (`KismetMathLibrary.RandomIntegerInRange` 1 4))
  (`KismetArrayLibrary.Array_Set` (`self.Shadow Dice`) 3 (`KismetMathLibrary.RandomIntegerInRange` 1 4))
  (`KismetArrayLibrary.Array_Set` (`self.Shadow Dice`) 2 (`KismetMathLibrary.RandomIntegerInRange` 1 64))
  (`KismetArrayLibrary.Array_Set` (`self.Shadow Dice`) 3 (`KismetMathLibrary.RandomIntegerInRange` 1 4))
  (return (`self.Shadow Dice`)))