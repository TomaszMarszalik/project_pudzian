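; BP_Tile is a clickable grid tile that supports square, point-top hexagon and flat-top hexagon layouts.
; Initialize sets the mesh for the given type, attaches the tile to its owner and positions it via CalculateLocation.
; CalculateLocation derives position from Row, Column and mesh bounds, staggering alternate hexagon rows or columns.
; Clicking moves the player character to the tile with SimpleMoveToLocation and draws debug text and a line.
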(event `self.ReceiveActorOnClicked`
  (params (ButtonPressed :type "Key Structure"))
  (bind _returnvalue (`GameplayStatics.GetPlayerCharacter` 0))
  (bind _returnvalue_2 (`ActorComponent.GetOwner` (`self.Tile`)))
  (bind (_returnvalue_x _returnvalue_y) (`KismetMathLibrary.BreakVector` (`self.K2_GetActorLocation` _returnvalue_2)))
  (bind _returnvalue_3 (`self.K2_GetActorLocation` _returnvalue_2))
  (`KismetSystemLibrary.PrintText` (`|FormatText` "{x} / {y}" _returnvalue_x _returnvalue_y))
  (`AIBlueprintHelperLibrary.SimpleMoveToLocation` (`Pawn.GetController` _returnvalue) _returnvalue_3)
  (`KismetSystemLibrary.PrintText` "Hello")
  (`KismetSystemLibrary.DrawDebugLine` (`self.K2_GetActorLocation` _returnvalue) _returnvalue_3 (struct :`R` 1.0 :`G` 0.161216 :`B` 0.362264 :`A` 1.0) 1.0 2.0))

(fn `CalculateLocation`
  (params (InType :type "/Game/Blueprints/EGridType Enum" :default "NewEnumerator0"))
  (returns (OutLocation :type "Vector Structure"))
  (bind _x (.x (`.BoxExtent` (`KismetSystemLibrary.GetComponentBounds` (`self.Tile`)))))
  (bind _y (.y (`.BoxExtent` (`KismetSystemLibrary.GetComponentBounds` (`self.Tile`)))))
  (bind _returnvalue (* _y 2.0 (`self.Row`)))
  (bind _returnvalue_2 (* _x 2.0 (`self.Column`)))
  (return (select `/Game/Blueprints/EGridType` InType :`NewEnumerator0` (`KismetMathLibrary.MakeVector` (* (.x (`.BoxExtent` (`KismetSystemLibrary.GetComponentBounds` (`self.Tile`)))) (`self.Column`)) (* (.y (`.BoxExtent` (`KismetSystemLibrary.GetComponentBounds` (`self.Tile`)))) (`self.Row`))) :`NewEnumerator1` (`KismetMathLibrary.MakeVector` (`KismetMathLibrary.SelectFloat` _returnvalue_2 (+ _returnvalue_2 _x) (== (mod (`self.Row`) 2) 0)) (* (.y (`.BoxExtent` (`KismetSystemLibrary.GetComponentBounds` (`self.Tile`)))) 2.0 (`self.Row`) (/ 3.0 4.0))) :`NewEnumerator2` (`KismetMathLibrary.MakeVector` (* (.x (`.BoxExtent` (`KismetSystemLibrary.GetComponentBounds` (`self.Tile`)))) 2.0 (`self.Column`) (/ 3.0 4.0)) (`KismetMathLibrary.SelectFloat` _returnvalue (+ _returnvalue _y) (== (mod (`self.Column`) 2) 0))))))

(fn `Initialize`
  (params (InType :type "/Game/Blueprints/EGridType Enum" :default "NewEnumerator0"))
  (bind _returnvalue (`self.GetOwner`))
  (`/Engine/EditorBlueprintResources/StandardMacros.IsValid` _returnvalue
    (:`Is Valid`
      (`self.SetMesh` InType)
      (`self.K2_AttachToActor` _returnvalue "None" "SnapToTarget" "KeepWorld" "KeepRelative" false)
      (bind _outlocation (`self.CalculateLocation` (`local.InType`)))
      (`self.K2_SetActorRelativeLocation` _outlocation))))

(fn `SetMesh`
  (params (InType :type "/Game/Blueprints/EGridType Enum" :default "NewEnumerator0"))
  (`StaticMeshComponent.SetStaticMesh` (`self.Tile`) (select `/Game/Blueprints/EGridType` InType :`NewEnumerator0` "/Engine/BasicShapes/Plane.Plane" :`NewEnumerator1` "/Game/Meshes/Hexagon_P_Top.Hexagon_P_Top" :`NewEnumerator2` "/Game/Meshes/Hexagon_F_Top.Hexagon_F_Top" :!type "StaticMesh Object Reference")))

(fn `UserConstructionScript`)